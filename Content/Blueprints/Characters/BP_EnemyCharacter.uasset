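; Enemy character that wields a sword, shows a camera-facing health bar and is tinted by EnemyColor through a dynamic material.
; BeginPlay spawns BP_Sword1 on the weapon's mesh socket; Attack plays a sword montage unless dead or already animating.
; Health component events refresh the bar on damage and, on death, award score through BP_MyGameMode, disable movement and collision, then destroy the actor after a delay.
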(event OnDamage(Health)
  (params (DamageAmount :type Float%20%28single-precision%29) (IsCrit :type Boolean))
  (CallFunction|SetHpBarPercentage))

(event OnDeath(Health)
  ;[0.5833 0.02442 0] On enemy death
  ;;[1 1 1] Increment score
  (Utilities|FlowControl|Sequence
    (:then_0
      (bind _asbp_my_game_mode (Utilities|Casting|CastToBP_MyGameMode (Game|GetGameMode)))
      (Default|IncreaseScore _asbp_my_game_mode (Variables|Default|GetScoreAmount)))
    (:then_1
      (Pawn|Components|CharacterMovement|DisableMovement (Variables|Character|GetCharacterMovement))
      (Collision|SetCollisionEnabled (Variables|Default|GetCapsuleComponent) "NoCollision")
      (Audio|SpawnSoundAttached "/Game/Audio/PlayerDeath.PlayerDeath" (Variables|Character|GetMesh) "None" "0, 0, 0" "0, 0, 0" "KeepRelativeOffset" false 1.0 1.0 0.0 0 0)
      (Utilities|FlowControl|Delay 3.0)
      (Actor|DestroyActor))))

(event Custom|DestroyWeapon
  (params (DestroyedActor :type Actor%20Object%20Reference))
  (CallFunction|DestroyCurrentWeapon))

(event Custom|Attack
  ;[1 0.5444 0.4409] Handle attack
  (if (not (Class|Health|IsDead (Variables|Default|GetHealth)))
    ;;[1 1 1] If no montage is currently playing
    (if (not (Animation|Montage|MontageIsPlaying (Components|SkeletalMesh|GetAnimInstance (Variables|Character|GetMesh)) 0))
      (Animation|Montage|PlayMontage (Variables|Character|GetMesh) "/Game/ImportedPacks/ShooterMannequin/Animations/AM_SwordHit.AM_SwordHit"))))

(event EventBeginPlay
  (|CallParentFunction)
  (CallFunction|EquipWeapon "/Game/Blueprints/Weapons/BP_Sword1.BP_Sword1_C")
  (Game|BindEventtoOnDestroyed (delegate Custom|DestroyWeapon))
  (CallFunction|SetHpBarPercentage))

(event EventTick
  (params (DeltaSeconds :type Float%20%28single-precision%29))
  (|CallParentFunction DeltaSeconds)
  (Class|FLookatCamera|LookatCamera (Variables|Default|GetHpBar) false false))

(fn ConstructionScript
  (|CallParentFunction)
  (bind _returnvalue (Rendering|Material|CreateDynamicMaterialInstance (Variables|Character|GetMesh) 0 0 "None" :!class /Script/Engine.PrimitiveComponent))
  (bind _output_get (Variables|Enemy|SetBodyMaterialInstance _returnvalue))
  (Rendering|Material|SetVectorParameterValue _output_get "BodyColor" (Variables|Enemy|GetEnemyColor) :!class /Script/Engine.MaterialInstanceDynamic))

(fn EquipWeapon
  (params (Weapon :type Base%20Weapon%20Class%20Reference))
  ;[1 1 1] If there is a current weapon, destroy it
  (bind _currentweapon (Variables|Default|GetCurrentWeapon)
    (:then
      (Actor|DestroyActor _currentweapon))
    (:else
      _))
  (bind _asbase_weapon (Utilities|Casting|CastToBaseWeaponClass (Class|KismetMathLibrary|SelectClass Weapon "/Script/EchoOfThePast.BaseWeapon" (Utilities|IsValidClass Weapon))))
  ;[1 1 1] Spawn and attach weapon
  (bind _returnvalue (Game|SpawnActorfromClass _asbase_weapon (Math|Transform|MakeTransform "0, 0, 0") "Undefined" "MultiplyWithRoot" 0 0))
  (bind _output_get (Variables|Default|SetCurrentWeapon _returnvalue))
  (Transformation|AttachComponentToComponent _output_get (Variables|Character|GetMesh) (Variables|/Script/EchoOfThePast.BaseWeapon|GetSocketName _returnvalue) "SnapToTarget" "SnapToTarget" "SnapToTarget" true))

(fn SetHpBarPercentage
  (bind _asbpw_health_bar (Utilities|Casting|CastToBPW_HealthBar (UserInterface|GetWidget (Variables|Default|GetHpBar))))
  (Variables|/Game/Blueprints/Widgets/BPW_HealthBar.BPW_HealthBar_C|SetHealthPercentage _asbpw_health_bar (Class|Health|GetHealthPercentage (Variables|Default|GetHealth))))