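; Player character with melee and ranged combat, dodge, sprint and a minimap widget.
; Attack type selects the equipped sword or gun, spawned onto a mesh socket; pickups update those slots.
; Attacks emit noise and call the weapon; melee plays random montages, gated by DoOnce like the cooldown-limited dodge, which faces movement input at run speed.
; On death it stops, then after a delay requests a game-mode respawn and destroys itself.
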(event OnDeath(Health)
  ;[0.5 0 0.003162] Handle player death
  (Pawn|Components|CharacterMovement|DisableMovement (Variables|Character|GetCharacterMovement))
  (bind _currentweapon (Variables|Default|GetCurrentWeapon)
    (:then
      (Class|BaseWeapon|Attack _currentweapon false))
    (:else
      _))
  (Utilities|FlowControl|Delay 3.0)
  (bind _asbp_my_game_mode (Utilities|Casting|CastToBP_MyGameMode (Game|GetGameMode)))
  (Default|RespawnPlayer _asbp_my_game_mode)
  (CallFunction|DestroyCurrentWeapon)
  (Actor|DestroyActor))

(event Custom|Dodge
  ;[1 1 1] Dodge
  (if (and (> (- (Utilities|Time|GetGameTimeinSeconds) (Variables|Movement|GetLastTimeDodged)) (Variables|Movement|GetDodgeInterval)) (not (Class|Health|IsDead (Variables|Default|GetHealth))))
    (Variables|Movement|SetLastTimeDodged (Utilities|Time|GetGameTimeinSeconds))
    (Utilities|FlowControl|DoOnce false :!label _label
      (:Completed
        (Variables|/Script/Engine.CharacterMovementComponent|SetMaxWalkSpeed (Variables|Character|GetCharacterMovement) (Variables|Movement|GetRunSpeed))
        (if (CallFunction|IsMoving)
          (Transformation|SetActorRotation (Math|Conversions|RotationFromXVector (Class|Pawn|GetLastMovementInputVector))))
        (Animation|Montage|PlayMontage (Variables|Character|GetMesh) "/Game/Animation/AnimMontages/AM_DodgeMontage.AM_DodgeMontage"
          (:OnCompleted
            (Variables|/Script/Engine.CharacterMovementComponent|SetMaxWalkSpeed (Variables|Character|GetCharacterMovement) (Variables|Movement|GetWalkSpeed)))
          (:OnBlendOut
            (goto _label Reset))
          (:OnInterrupted
            (goto _label Reset)))))))

(event Custom|StartSprint
  (params (IsStart :type Boolean))
  (bind _charactermovement (Variables|Character|GetCharacterMovement))
  ;[1 1 1] Handle sprint actions
  (if IsStart
    (Variables|/Script/Engine.CharacterMovementComponent|SetMaxWalkSpeed _charactermovement (Variables|Movement|GetRunSpeed))
    (else
      (Variables|/Script/Engine.CharacterMovementComponent|SetMaxWalkSpeed _charactermovement (Variables|Movement|GetWalkSpeed)))))

(event Custom|Attack
  (params (IsStart :type Boolean))
  ;[1 0.5444 0.4409] Handle attack
  (if (not (Class|Health|IsDead (Variables|Default|GetHealth)))
    (if (not (Animation|Montage|MontageIsPlaying (Components|SkeletalMesh|GetAnimInstance (Variables|Character|GetMesh)) "/Game/Animation/AnimMontages/AM_DodgeMontage.AM_DodgeMontage"))
      (switch Utilities|FlowControl|Switch|SwitchonEDamageType (Variables|Attack|GetAttackType)
        (:NewEnumerator0
          (Utilities|FlowControl|DoOnce false :!label _label
            (:Completed
              (Class|Actor|MakeNoise 0.5 0 "0, 0, 0" 0.0 "None")
              (bind _asbase_melee_weapon (Utilities|Casting|CastToBaseMeleeWeapon (Variables|Default|GetCurrentWeapon))
                (:then
                  (Animation|Montage|PlayMontage (Variables|Character|GetMesh) (Utilities|Select :Index (Math|Random|RandomInteger 3) :Option%200 "/Game/Animation/AnimMontages/AM_SwordHit.AM_SwordHit" :Option%201 "/Game/Animation/AnimMontages/AM_MeleeAttack2.AM_MeleeAttack2" :Option%202 "/Game/Animation/AnimMontages/AM_MeleeAttack3.AM_MeleeAttack3") (Class|BaseMeleeWeapon|GetPlayRate _asbase_melee_weapon)
                    (:then
                      _)
                    (:OnCompleted
                      (goto _label Reset))
                    (:OnBlendOut
                      (goto _label Reset))
                    (:OnInterrupted
                      ;;[1 1 1] In case it gets interrupted, reset
                      (Utilities|FlowControl|Delay 1.0 :!label _label_2)
                      (goto _label Reset))))
                (:CastFailed
                  (Animation|Montage|PlayMontage (Variables|Character|GetMesh) (Utilities|Select :Index (Math|Random|RandomInteger 3) :Option%200 "/Game/Animation/AnimMontages/AM_Punch1.AM_Punch1" :Option%201 "/Game/Animation/AnimMontages/AM_Punch2.AM_Punch2" :Option%202 "/Game/Animation/AnimMontages/AM_Punch3.AM_Punch3")
                    (:then
                      _)
                    (:OnCompleted
                      (goto _label Reset))
                    (:OnBlendOut
                      (goto _label Reset))
                    (:OnInterrupted
                      (goto _label_2)))))
              (bind _currentweapon (Variables|Default|GetCurrentWeapon)
                (:then
                  (Class|BaseWeapon|Attack _currentweapon true))
                (:else)))))
        (:NewEnumerator1
          (Class|Actor|MakeNoise 1.0 0 "0, 0, 0" 0.0 "None")
          (bind _currentweapon_2 (Variables|Default|GetCurrentWeapon)
            (:then
              (Class|BaseWeapon|Attack _currentweapon_2 IsStart))
            (:else)))))))

(event Custom|ResetAttack
  ;[1 0.5444 0.4409] Handle attack
  (Utilities|FlowControl|DoOnce false) ; enters at Reset
)

(event Custom|SwitchAttackType
  (params (NewParam :type EDamageType%20Enum :default "NewEnumerator0"))
  ;[1 1 1] Switch attack event
  (bind _output_get (Variables|Attack|SetAttackType NewParam))
  (switch Utilities|FlowControl|Switch|SwitchonEDamageType _output_get
    (:NewEnumerator0
      (CallFunction|SwitchWeapon (Variables|Attack|GetEquippedSword)))
    (:NewEnumerator1
      (CallFunction|SwitchWeapon (Variables|Attack|GetEquippedGun)))))

(event EventBeginPlay
  ;[0.4462 0.4462 0.4462] Begin play actions
  (|CallParentFunction)
  ;;[1 1 1] Set walk and run speed
  (bind _output_get (Variables|Movement|SetWalkSpeed (Variables|/Script/Engine.CharacterMovementComponent|GetMaxWalkSpeed (Variables|Character|GetCharacterMovement))))
  (Variables|Movement|SetRunSpeed (* _output_get 1.5))
  (CallFunction|SwitchWeapon (Variables|Attack|GetEquippedGun))
  (bind _returnvalue (UserInterface|CreateWidget "/Game/Blueprints/Widgets/W_Minimap.W_Minimap_C" (Game|GetPlayerController 0)))
  (UserInterface|Viewport|AddtoViewport _returnvalue 0))

(fn ConstructionScript
  (|CallParentFunction))

(fn IsMoving
  (return (> (Math|Vector|VectorLengthSquared (Transformation|GetVelocity)) 0.0)))

(fn SwitchWeapon
  (params (WeaponRef :type Base%20Weapon%20Class%20Reference))
  ;[1 1 1] If there is a current weapon, destroy it
  (bind _currentweapon (Variables|Default|GetCurrentWeapon)
    (:then
      (Actor|DestroyActor _currentweapon))
    (:else
      _))
  ;[1 1 1] Spawn and attach weapon
  (bind _asbase_weapon (Utilities|Casting|CastToBaseWeaponClass (Class|KismetMathLibrary|SelectClass WeaponRef "/Script/EchoOfThePast.BaseWeapon" (Utilities|IsValidClass WeaponRef))))
  (bind _returnvalue (Game|SpawnActorfromClass _asbase_weapon (Math|Transform|MakeTransform "0, 0, 0") "Undefined" "MultiplyWithRoot" 0 0))
  (bind _output_get (Variables|Default|SetCurrentWeapon _returnvalue))
  (Transformation|AttachComponentToComponent _output_get (Variables|Character|GetMesh) (Variables|/Script/EchoOfThePast.BaseWeapon|GetSocketName _returnvalue) "SnapToTarget" "SnapToTarget" "SnapToTarget" true))

(fn EquipWeapon
  (params (WeaponRef :type Base%20Weapon%20Class%20Reference) (WeaponType :type EDamageType%20Enum :default "NewEnumerator0"))
  ;[1 1 1] If the current weapon is of the same time as the pick up, switch weapon immediately
  (if (Utilities|Enum|Equal(Enum) WeaponType (Variables|Attack|GetAttackType))
    (CallFunction|SwitchWeapon WeaponRef))
  (switch Utilities|FlowControl|Switch|SwitchonEDamageType WeaponType
    (:NewEnumerator0
      (Variables|Attack|SetEquippedSword WeaponRef))
    (:NewEnumerator1
      (Variables|Attack|SetEquippedGun WeaponRef))))