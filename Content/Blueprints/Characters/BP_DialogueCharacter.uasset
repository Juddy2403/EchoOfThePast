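; Talkable NPC that plays its configured dialogue when interacted with and shows a name label and quest markers.
; On BeginPlay it copies its text, name and audio into the dialogue actor component, which handles talking on Interact.
; When the component signals that dialogue is over, both quest icons are hidden.
; The construction script sets the name label from CharName.
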(event OnDialogueOver(BP_Dialogue_AC)
  ;[1 1 1] Hide exclamation mark when dialogue is over
  (Rendering|SetVisibility (Variables|Default|GetSPR_QuestIcon1) false false))

(event EventBeginPlay
  (bind _bp_dialogue_ac (Variables|Default|GetBP_Dialogue_AC))
  ;[1 1 1] Initialize dialogue
  (Variables|/Game/Blueprints/Components/BP_Dialogue_AC.BP_Dialogue_AC_C|SetDialogueText _bp_dialogue_ac (Variables|Dialogue|GetDialogue%20Text))
  (Variables|/Game/Blueprints/Components/BP_Dialogue_AC.BP_Dialogue_AC_C|SetCharName _bp_dialogue_ac (Variables|Dialogue|GetChar%20Name))
  (Variables|/Game/Blueprints/Components/BP_Dialogue_AC.BP_Dialogue_AC_C|SetDialogueAudio _bp_dialogue_ac (Variables|Dialogue|GetDialogueAudio)))

(event EventInteract
  ;[1 1 1] Talk when interacted with
  (Class|DialogueInterface|Talk (Variables|Default|GetBP_Dialogue_AC)))

(fn ConstructionScript
  (Rendering|Components|TextRender|SetText (Variables|Default|GetName) (Utilities|Text|ToText(String) (Variables|Dialogue|GetChar%20Name))))