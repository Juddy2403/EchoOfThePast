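; Base character Blueprint that gives hit feedback and can destroy its current weapon.
; When the Health component reports damage on a living character, it draws floating damage with crit info and, for positive damage, flickers the body color.
; Flicker uses a DoOnce-gated timeline to lerp a dynamic material parameter between red and its original color, then restores it.
; Random hit-react montage logic exists but is disconnected.
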(event OnDamage(Health)
  (params (DamageAmount :type Float%20%28single-precision%29) (IsCrit :type Boolean))
  (bind _bpc_floatingdamage (Variables|Default|GetBPC_FloatingDamage))
  ;[1 0.8015 0.2969] Draw floating damage
  (if (not (Class|Health|IsDead (Variables|Default|GetHealth)))
    (Default|InitData _bpc_floatingdamage DamageAmount IsCrit)
    (Default|DrawFloatingDamage _bpc_floatingdamage (Transformation|GetWorldLocation (Variables|Default|GetFloatingDamageSpawn)))
    (if (> DamageAmount 0.0)
      ;[0.5104 0.006962 0] Flicker and play hit animation
      (CallFunction|Flicker "BodyColor" 2.0))))

(event Custom|Flicker
  (params (DynMatColor :type Name) (PlayRate :type Float%20%28double-precision%29))
  ;[1 1 1] Flicker event
  (Components|Timeline|SetPlayRate (Variables|Default|GetFlickerTimeline) PlayRate)
  (Utilities|FlowControl|DoOnce false :!label _label
    (:Completed
      (bind _returnvalue (Rendering|Material|CreateDynamicMaterialInstance (Variables|Character|GetMesh) 0 0 DynMatColor :!class /Script/Engine.PrimitiveComponent))
      (Utilities|FlowControl|Sequence
        (:then_0
          (bind _returnvalue_2 (Rendering|Material|GetVectorParameterValue _returnvalue DynMatColor :!class /Script/Engine.MaterialInstanceDynamic)))
        (:then_1
          (bind _flickerstate (Timeline|FlickerTimeline PlayFromStart)
            (:Update
              (Rendering|Material|SetVectorParameterValue _returnvalue DynMatColor (Math|Color|Lerp(LinearColor) "(R=1.000000,G=0.010132,B=0.000000,A=1.000000)" _returnvalue_2 _flickerstate) :!class /Script/Engine.MaterialInstanceDynamic))
            (:Finished
              (Rendering|Material|SetVectorParameterValue _returnvalue DynMatColor _returnvalue_2 :!class /Script/Engine.MaterialInstanceDynamic)
              (goto _label Reset))))))))

(event Custom|DestroyCurrentWeapon
  (bind _currentweapon (Variables|Default|GetCurrentWeapon)
    (:then
      (Actor|DestroyActor _currentweapon))
    (:else)))

(fn ConstructionScript)