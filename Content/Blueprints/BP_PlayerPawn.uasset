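; BP_PlayerPawn is a player pawn that moves by consumed movement input and turns to face its direction of travel.
; Each tick it offsets itself with sweep by the input vector scaled by delta time and MovementSpeed.
; Nonzero movement updates DesiredRotation, and the pawn lerps toward it along the shortest path using delta time times RotationSpeed.
; The graph only consumes input; it contains no input bindings.
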(event EventBeginPlay)

(event Collision|EventActorBeginOverlap
  (params (OtherActor :type Actor%20Object%20Reference)))

(event EventTick
  (params (DeltaSeconds :type Float%20%28single-precision%29))
  ;[1 1 1] Movement
  (bind _returnvalue (Class|Pawn|ConsumeMovementInputVector))
  (Transformation|AddActorWorldOffset (* _returnvalue DeltaSeconds (Variables|PawnMovement|GetMovementSpeed)) true)
  ;[1 1 1] Calculate desired rotation
  (if (> (Math|Vector|VectorLengthSquared (* _returnvalue DeltaSeconds (Variables|PawnMovement|GetMovementSpeed))) 0.0)
    (Variables|PawnMovement|SetDesiredRotation (Math|Conversions|RotationFromXVector (* _returnvalue DeltaSeconds (Variables|PawnMovement|GetMovementSpeed)))))
  ;[0.1094 0.08421 0.1875 0.993 17] Rotate pawn to desired rotation
  (Transformation|SetActorRotation (Math|Rotator|Lerp(Rotator) (Transformation|GetActorRotation) (Variables|PawnMovement|GetDesiredRotation) (* DeltaSeconds (Variables|PawnMovement|GetRotationSpeed)) true)))

(fn ConstructionScript)