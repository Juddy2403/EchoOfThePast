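; Base character Blueprint that gives visual feedback when its BPC_Health component reports damage.
; On damage, a reusable Flicker event creates a dynamic material on the mesh and uses a timeline to lerp a named color parameter between red and its original value, restoring it afterward.
; It also plays a random hit-react montage, with DoOnce gates keeping flicker and montage from retriggering until each finishes.
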(event OnDamage(BPC_Health)
  (CallFunction|Flicker "BodyColor" 2.0)
  (Utilities|FlowControl|DoOnce false :!label _label
    (:Completed
      (Animation|Montage|PlayMontage (Variables|Character|GetMesh) (Utilities|Select :Index (Math|Random|RandomInteger 5) :Option%200 "/Game/ShooterMannequin/Animations/Hit_React_1_Montage.Hit_React_1_Montage" :Option%201 "/Game/ShooterMannequin/Animations/Hit_React_2_Montage.Hit_React_2_Montage" :Option%202 "/Game/ShooterMannequin/Animations/Hit_React_3_Montage.Hit_React_3_Montage" :Option%203 "/Game/ShooterMannequin/Animations/Hit_React_4_Montage.Hit_React_4_Montage" :Option%204 "/Game/ShooterMannequin/Animations/HitReact_Montage.HitReact_Montage")
        (:OnCompleted
          (goto _label Reset))))))

(event Custom|Flicker
  (params (DynMatColor :type Name) (PlayRate :type Float%20%28double-precision%29))
  ;[1 1 1] Flicker event
  (Components|Timeline|SetPlayRate (Variables|Default|GetFlickerTimeline) PlayRate)
  (Utilities|FlowControl|DoOnce false :!label _label
    (:Completed
      (bind _returnvalue (Rendering|Material|CreateDynamicMaterialInstance (Variables|Character|GetMesh) 0 0 DynMatColor :!class /Script/Engine.PrimitiveComponent))
      (Utilities|FlowControl|Sequence
        (:then_0
          (bind _returnvalue_2 (Rendering|Material|GetVectorParameterValue _returnvalue DynMatColor :!class /Script/Engine.MaterialInstanceDynamic)))
        (:then_1
          (bind _flickerstate (Timeline|FlickerTimeline PlayFromStart)
            (:Update
              (Rendering|Material|SetVectorParameterValue _returnvalue DynMatColor (Math|Color|Lerp(LinearColor) "(R=1.000000,G=0.010132,B=0.000000,A=1.000000)" _returnvalue_2 _flickerstate) :!class /Script/Engine.MaterialInstanceDynamic))
            (:Finished
              (Rendering|Material|SetVectorParameterValue _returnvalue DynMatColor _returnvalue_2 :!class /Script/Engine.MaterialInstanceDynamic)
              (goto _label Reset))))))))

(fn ConstructionScript)