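; BP_EnemyCharacter is an enemy character that damages the player on contact and awards score when killed.
; Player overlap starts a looping timer that damages the player's health component, and ending overlap clears it.
; Its health component's death event increments the game mode score, disables movement, attacks and collision, plays a sound, then destroys the actor after a delay.
; The construction script tints the body through a dynamic material instance.
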(event OnDeath(BPC_Health)
  ;[0.5833 0.02442 0] On enemy death
  ;;[1 1 1] Increment score
  (Utilities|FlowControl|Sequence
    (:then_0
      (bind _asbp_my_game_mode (Utilities|Casting|CastToBP_MyGameMode (Game|GetGameMode)))
      (Default|IncreaseScore _asbp_my_game_mode (Variables|Default|GetScoreAmount)))
    (:then_1
      (Pawn|Components|CharacterMovement|DisableMovement (Variables|Character|GetCharacterMovement))
      (Utilities|Time|ClearTimerbyFunctionName 0 "DamageCurrentPlayer")
      (Collision|SetCollisionEnabled (Variables|Default|GetDamageVolume) "NoCollision")
      (Collision|SetCollisionEnabled (Variables|Default|GetCapsuleComponent) "NoCollision")
      (Audio|SpawnSoundAttached "/Game/Audio/PlayerDeath.PlayerDeath" (Variables|Character|GetMesh) "None" "0, 0, 0" "0, 0, 0" "KeepRelativeOffset" false 1.0 1.0 0.0 0 0)
      (Utilities|FlowControl|Delay 3.0)
      (Actor|DestroyActor))))

(event Custom|DamageCurrentPlayer
  (bind _currentplayertarget (Variables|Damage|GetCurrentPlayerTarget))
  ;[1 1 1] Detect player collision
  ;;[1 0.3614 0.2516] Damage player while colliding
  (Utilities|IsValid _currentplayertarget
    (:Is%20Valid
      (Default|DoDamage (Variables|/Game/Blueprints/BP_BaseCharacter.BP_BaseCharacter_C|GetBPC_Health _currentplayertarget) (Variables|Damage|GetDamageAmount)))))

(event EventBeginPlay
  (|CallParentFunction) ; This node is disabled and will not be called.\nDrag off pins to build functionality.
)

(event Collision|EventActorBeginOverlap
  (params (OtherActor :type Actor%20Object%20Reference))
  ;[1 1 1] Detect player collision
  (|CallParentFunction OtherActor)
  (bind _asbp_player_character (Utilities|Casting|CastToBP_PlayerCharacter OtherActor))
  (Variables|Damage|SetCurrentPlayerTarget _asbp_player_character)
  (Utilities|Time|SetTimerbyEvent (delegate Custom|DamageCurrentPlayer) (Variables|Damage|GetAttackInterval) true))

(event EventTick
  (params (DeltaSeconds :type Float%20%28single-precision%29))
  (|CallParentFunction DeltaSeconds) ; This node is disabled and will not be called.\nDrag off pins to build functionality.
)

(event Collision|EventActorEndOverlap
  (params (OtherActor :type Actor%20Object%20Reference))
  ;[1 1 1] Detect player collision loss
  (if (== OtherActor (Variables|Damage|GetCurrentPlayerTarget))
    (Utilities|Time|ClearTimerbyFunctionName 0 "DamageCurrentPlayer")))

(fn ConstructionScript
  (|CallParentFunction)
  (bind _returnvalue (Rendering|Material|CreateDynamicMaterialInstance (Variables|Character|GetMesh) 0 0 "None" :!class /Script/Engine.PrimitiveComponent))
  (bind _output_get (Variables|Enemy|SetBodyMaterialInstance _returnvalue))
  (Rendering|Material|SetVectorParameterValue _output_get "BodyColor" (Variables|Enemy|GetEnemyColor) :!class /Script/Engine.MaterialInstanceDynamic))