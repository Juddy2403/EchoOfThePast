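; Game mode that runs level flow, pausing and the level timer.
; Reload restarts the current map (or L_Level2_1 for Level2 maps), while LevelConfig table rows keyed by map name set the next level, timer use and stat carry-over through the game instance.
; Player death, time-up and the controller's pause command feed one pause handler that broadcasts pause events.
; A separate OpenLevel event saves stats and delays loading for a transition.
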(event OnTimeUp(BP_Timer_AC)
  (CallFunction|SetGamePaused true))

(event On60SecRemaining(BP_Timer_AC)
  ;[1 1 1] Time almost up text
  (Default|ShowText (Variables|Default|GetBP_DisplayText_AC)))

(event Custom|ReloadLevel
  ;[1 1 1] Player died: respawn
  (bind _returnvalue (Game|GetCurrentLevelName true))
  ;;[1 1 1] Always load the first map of the second level
  (if (Utilities|String|Contains _returnvalue "L_Level2")
    (Game|OpenLevel(byName) "L_Level2_1")
    (else
      (Game|OpenLevel(byName) (Utilities|String|StringToName _returnvalue)))))

(event Custom|PauseGame
  (CallFunction|SetGamePaused true))

(event Custom|SetGamePaused
  (params (IsPaused :type Boolean))
  ;[1 1 1] Handle pausing logic
  (if IsPaused
    (Default|CallOnPaused)
    (Utilities|FlowControl|DelayUntilNextTick)
    (else
      (Default|CallOnUnpaused)))
  (Game|SetGamePaused IsPaused))

(event Custom|LoadNextLevel
  (bind _returnvalue (Game|GetCurrentLevelName true))
  (bind _returnvalue_2 (Utilities|GetDataTableRow (Variables|Default|GetLevelConfig) (Utilities|String|StringToName _returnvalue))
    (:then
      ;[1 1 1] Configure the next level settings
      (Utilities|FlowControl|Sequence
        (:then_0
          (if (.ShouldKeepPlayerStats (Utilities|Struct|BreakSLevelConfig _returnvalue_2))
            (bind _asbp_my_game_instance (Utilities|Casting|CastToBP_MyGameInstance (Game|GetGameInstance)))
            (Default|BindSetPlayerStatsEvent _asbp_my_game_instance)
            (Variables|/Game/Blueprints/GameInstances/BP_MyGameInstance.BP_MyGameInstance_C|SetRemainingTime _asbp_my_game_instance (Variables|/Game/Blueprints/Components/BP_Timer_AC.BP_Timer_AC_C|GetRemainingTime (Variables|Default|GetBP_Timer_AC)))))
        (:then_1
          (CallFunction|OpenLevel (.NextLevelName (Utilities|Struct|BreakSLevelConfig _returnvalue_2))))))
    (:RowNotFound
      (Development|PrintString "Load next level- row not found" true true "(R=1.000000,G=0.009549,B=0.000000,A=1.000000)"))))

(event Custom|OpenLevel
  (params (LevelName :type Name))
  ;[1 1 1] Open level and play black screen animation
  (Utilities|FlowControl|Sequence
    (:then_0
      (bind _asbp_my_game_instance (Utilities|Casting|CastToBP_MyGameInstance (Game|GetGameInstance)))
      (Default|SetPlayerStats _asbp_my_game_instance))
    (:then_1
      (Default|CallOnOpenLevelTransition)
      (Utilities|FlowControl|Delay 1.0)
      (Game|OpenLevel(byName) LevelName))
    (:then_2
      (if (Game|IsGamePaused)
        (CallFunction|SetGamePaused false)))))

(event EventBeginPlay
  (Utilities|FlowControl|Sequence
    (:then_0
      (bind _asbp_my_game_instance (Utilities|Casting|CastToBP_MyGameInstance (Game|GetGameInstance)))
      (Default|CallOnLevelLoaded _asbp_my_game_instance))
    (:then_1
      (bind _asbp_player_character (Utilities|Casting|CastToBP_PlayerCharacter (Game|Player|GetPlayerPawn 0)))
      (EventDispatchers|BindEventtoOnPlayerDeath _asbp_player_character (delegate Custom|PauseGame)))
    (:then_2
      ;[1 1 1] Smooth black->level transition animation
      (bind _asbp_player_controller (Utilities|Casting|CastToBP_PlayerController (Game|GetPlayerController 0)))
      (EventDispatchers|BindEventtoOnPauseCommand _asbp_player_controller (delegate Custom|SetGamePaused)))
    (:then_3
      (bind _returnvalue (Game|GetCurrentLevelName true))
      (bind _returnvalue_2 (Utilities|GetDataTableRow (Variables|Default|GetLevelConfig) (Utilities|String|StringToName _returnvalue))
        (:then
          (if (not (.HasTimer (Utilities|Struct|BreakSLevelConfig _returnvalue_2)))
            (Default|Disable (Variables|Default|GetBP_Timer_AC))))))))

(fn ConstructionScript)