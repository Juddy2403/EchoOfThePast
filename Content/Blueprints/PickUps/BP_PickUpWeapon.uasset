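; Weapon pickup that equips its weapon on the player character when interacted with, then disables itself (hidden, no tick, collision or physics).
; An overlap collider toggles a camera-facing W_WeaponStats widget for the player.
; It binds to the player's OnPickUp dispatcher, so a disabled pickup with a matching weapon type re-enables above the player as a dropped weapon, reusing the actor instead of respawning it.
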(event OnComponentBeginOverlap(WidgetShowCollider)
  (params (OverlappedComponent :type Primitive%20Component%20Object%20Reference) (OtherActor :type Actor%20Object%20Reference) (OtherComp :type Primitive%20Component%20Object%20Reference) (OtherBodyIndex :type Integer) (bFromSweep :type Boolean) (SweepResult :type Hit%20Result%20Structure%20%28by%20ref%29))
  (bind _widget (Variables|Default|GetWidget))
  ;[0.4424 0.5654 1] Handle stats widget
  (if (== OtherActor (Game|GetPlayerCharacter 0))
    (Development|SetHiddeninGame _widget false false)
    (bind _asw_weapon_stats (Utilities|Casting|CastToW_WeaponStats (UserInterface|GetUserWidgetObject _widget)))
    (Default|SetStats _asw_weapon_stats (Variables|Default|GetWeaponType))))

(event OnComponentEndOverlap(WidgetShowCollider)
  (params (OverlappedComponent :type Primitive%20Component%20Object%20Reference) (OtherActor :type Actor%20Object%20Reference) (OtherComp :type Primitive%20Component%20Object%20Reference) (OtherBodyIndex :type Integer))
  ;[0.4424 0.5654 1] Handle stats widget
  (if (== (Game|GetPlayerCharacter 0) OtherActor)
    (Development|SetHiddeninGame (Variables|Default|GetWidget) true false)))

(event Custom|OnPickUp
  (params (WeaponType :type EDamageType%20Enum :default "NewEnumerator0"))
  ;[1 1 1] On weapon picked up, drop this pick up if it was previously equiped by the player
  (if (and (Variables|Default|GetIsDisabled) (Utilities|Enum|Equal(Enum) WeaponType (Variables|Default|GetWeaponType)))
    (CallFunction|ChangeStatus true)
    (Transformation|SetActorLocation (+ (Transformation|GetActorLocation (Game|Player|GetPlayerPawn 0)) "0.000000,0.000000,100.000000") false false)))

(event EventBeginPlay
  ;[0.4402 1 0.3416] Initialize stats widget
  (bind _asw_weapon_stats (Utilities|Casting|CastToW_WeaponStats (UserInterface|GetUserWidgetObject (Variables|Default|GetWidget))))
  (Default|SetInitStats _asw_weapon_stats (Variables|Default|GetWeaponRef) (Variables|Default|GetWeaponType))
  (bind _asbp_player_character (Utilities|Casting|CastToBP_PlayerCharacter (Game|GetPlayerCharacter 0)))
  (EventDispatchers|AssignOnPickUp _asbp_player_character (delegate Custom|OnPickUp)))

(event EventInteract
  ;[1 0.9694 0.2631] Switch weapon when pressing E
  (bind _asbp_player_character (Utilities|Casting|CastToBP_PlayerCharacter (Game|GetPlayerCharacter 0)))
  (Default|EquipWeapon _asbp_player_character (Variables|Default|GetWeaponRef) (Variables|Default|GetWeaponType))
  ;;[1 0.4027 0.3595] Disable actor while equipped by player
  (CallFunction|ChangeStatus false))

(event EventTick
  (params (DeltaSeconds :type Float%20%28single-precision%29))
  (bind _widget (Variables|Default|GetWidget))
  ;[1 1 1] Face widget towards camera
  (if (not (Variables|/Script/Engine.SceneComponent|GetbHiddenInGame _widget))
    (Class|FLookatCamera|LookatCamera _widget false false)))

(fn ConstructionScript
  (|CallParentFunction))

(fn ChangeStatus
  (params (Enabled :type Boolean))
  (bind _returnvalue (not Enabled))
  (Actor|Tick|SetActorTickEnabled Enabled)
  (Physics|SetSimulatePhysics (Variables|Default|GetCollisionDetection) Enabled)
  (Collision|SetActorEnableCollision Enabled)
  (Rendering|SetActorHiddenInGame _returnvalue)
  (Variables|Default|SetIsDisabled _returnvalue))