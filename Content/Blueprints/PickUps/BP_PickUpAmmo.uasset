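; Ammo pickup actor that gives the player ammunition when interacted with.
; Interact casts the player character, passes Ammo to AddAmmo, plays an equip sound at the CollisionDetection component and destroys the actor.
; ChangeStatus enables or disables the pickup by toggling tick, physics simulation, collision and visibility together, and records the state in IsDisabled.
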(event EventInteract
  ;[1 0.9694 0.2631] Switch weapon when pressing E
  (bind _asbp_player_character (Utilities|Casting|CastToBP_PlayerCharacter (Game|GetPlayerCharacter 0)))
  (Default|AddAmmo _asbp_player_character (Variables|Default|GetAmmo))
  (Audio|SpawnSoundatLocation "/Game/Audio/SoundWaves/A_ItepEquipped.A_ItepEquipped" (Transformation|GetWorldLocation (Variables|Default|GetCollisionDetection)) "0, 0, 0" 1.0 1.0 0.0 0 0)
  (Actor|DestroyActor))

(fn ConstructionScript
  (|CallParentFunction))

(fn ChangeStatus
  (params (Enabled :type Boolean))
  (bind _returnvalue (not Enabled))
  (Actor|Tick|SetActorTickEnabled Enabled)
  (Physics|SetSimulatePhysics (Variables|Default|GetCollisionDetection) Enabled)
  (Collision|SetActorEnableCollision Enabled)
  (Rendering|SetActorHiddenInGame _returnvalue)
  (Variables|Default|SetIsDisabled _returnvalue))