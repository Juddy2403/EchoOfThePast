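; BP_HealPotion is a health pickup that heals the player character when interacted with.
; On Interact it casts player 0's character to BP_PlayerCharacter, then spawns a spark particle effect and a pickup sound at that character's location.
; It passes HealAmount to the character's Health.Heal and destroys itself, so it is single-use.
; The construction script only calls the parent version.
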(event EventInteract
  ;[0.3896 1 0.4575] Heal character when pressing E
  (bind _asbp_player_character (Utilities|Casting|CastToBP_PlayerCharacter (Game|GetPlayerCharacter 0)))
  (Effects|SpawnEmitteratLocation "/Game/ImportedPacks/Realistic_Starter_VFX_Pack_Vol2/Particles/Sparks/P_Sparks_B.P_Sparks_B" (Transformation|GetActorLocation _asbp_player_character))
  (Audio|SpawnSoundatLocation "/Game/Audio/SoundWaves/A_HealthPickup.A_HealthPickup" (Transformation|GetActorLocation _asbp_player_character) "0, 0, 0" 1.0 1.0 0.0 0 0)
  (Class|Health|Heal (Variables|/Game/Blueprints/Characters/BP_BaseCharacter.BP_BaseCharacter_C|GetHealth _asbp_player_character) (Variables|Default|GetHealAmount))
  (Actor|DestroyActor))

(fn ConstructionScript
  (|CallParentFunction))