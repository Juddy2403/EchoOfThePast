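; Sci-fi sword weapon that damages what its blade touches when the Attack event is called.
; Attack sphere-traces between the mesh's Start and End sockets with debug drawing on, skipping actors that carry the ignore tag.
; Damage goes through BPI_Damageable to both the hit actor and each of its implementing components, playing an attached impact sound each time.
; The component loop stops if the actor becomes invalid.
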(event Custom|Attack
  (bind _weaponmesh (Variables|Default|GetWeaponMesh))
  ;[0.3073 0.2208 0.2198] Handle attacking
  (bind _outhit (Collision|SphereTraceForObjects (Transformation|GetSocketLocation _weaponmesh "Start") (Transformation|GetSocketLocation _weaponmesh "End") 5.0 (Utilities|Array|MakeArray "ObjectTypeQuery2" "ObjectTypeQuery3") false 0 "ForDuration"))
  (Utilities|IsValid (.HitActor (Collision|BreakHitResult _outhit))
    (:Is%20Valid
      (if (not (Actor|ActorHasTag (.HitActor (Collision|BreakHitResult _outhit)) (Variables|Default|GetIgnoreTag)))
        (Utilities|FlowControl|Sequence
          (:then_0
            ;;[1 1 1] Does the object itself implement the interface?
            (if (Utilities|DoesObjectImplementInterface (.HitActor (Collision|BreakHitResult _outhit)) "/Game/Blueprints/BPI_Damageable.BPI_Damageable_C")
              (Class|BPIDamageable|DoDamage(Message) (.HitActor (Collision|BreakHitResult _outhit)) (Variables|Default|GetDamageAmount))
              (Audio|SpawnSoundAttached "/Game/Audio/234082__211redman112__lasgun-impact.234082__211redman112__lasgun-impact" (Variables|Default|GetWeaponMesh) "None" "0, 0, 0" "0, 0, 0" "KeepRelativeOffset" false 1.0 1.0 0.0 0 0)))
          (:then_1
            ;;[1 1 1] Get all Components that implement the BPI_Damageable interfere and do damage
            (bind _index (Utilities|FlowControl|ForLoopwithBreak 0 (- (Utilities|Array|Length (Class|Actor|GetComponentsbyInterface (.HitActor (Collision|BreakHitResult _outhit)) "/Game/Blueprints/BPI_Damageable.BPI_Damageable_C")) -1) :!label _label)
              (:LoopBody
                (Class|BPIDamageable|DoDamage(Message) (Utilities|Array|Get(acopy) (Class|Actor|GetComponentsbyInterface (.HitActor (Collision|BreakHitResult _outhit)) "/Game/Blueprints/BPI_Damageable.BPI_Damageable_C") _index) (Variables|Default|GetDamageAmount))
                (Audio|SpawnSoundAttached "/Game/Audio/234082__211redman112__lasgun-impact.234082__211redman112__lasgun-impact" (Variables|Default|GetWeaponMesh) "None" "0, 0, 0" "0, 0, 0" "KeepRelativeOffset" false 1.0 1.0 0.0 0 0)
                (Utilities|IsValid (.HitActor (Collision|BreakHitResult _outhit))
                  (:Is%20Not%20Valid
                    (goto _label Break)))))))))))

(event EventBeginPlay
  (|CallParentFunction) ; This node is disabled and will not be called.\nDrag off pins to build functionality.
)

(event Collision|EventActorBeginOverlap
  (params (OtherActor :type Actor%20Object%20Reference))
  (|CallParentFunction OtherActor) ; This node is disabled and will not be called.\nDrag off pins to build functionality.
)

(event EventTick
  (params (DeltaSeconds :type Float%20%28single-precision%29)))

(fn ConstructionScript
  (|CallParentFunction))