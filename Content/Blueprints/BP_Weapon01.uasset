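; BP_Weapon01 is a child weapon Blueprint that provides automatic primary fire by overriding the parent's Fire event.
; Pressing fire shoots instantly, then starts a looping timer at the primary fire rate, guarded by a DoOnce.
; Each shot plays a blaster sound, prints debug text and spawns the primary projectile at FireSocket.
; Release clears the timer and resets the DoOnce, so repeated presses are not rate-limited here.
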(event Custom|SpawnPrimaryProjectile
  ;[1 1 1] Handle Fire
  (Audio|SpawnSoundAttached "/Game/Audio/466867__mikee63__blaster-shot-single-5.466867__mikee63__blaster-shot-single-5" (Variables|Default|GetWeaponMesh) "None" "0, 0, 0" "0, 0, 0" "KeepRelativeOffset" false 1.0 1.0 0.0 0 0)
  (Development|PrintString "Primary pew")
  (Game|SpawnActorfromClass (Variables|Default|GetPrimaryProjectileClass) (Transformation|GetWorldTransform (Variables|Default|GetFireSocket)) "Undefined" "MultiplyWithRoot" 0 0))

(event EventBeginPlay
  (|CallParentFunction) ; This node is disabled and will not be called.\nDrag off pins to build functionality.
)

(event Collision|EventActorBeginOverlap
  (params (OtherActor :type Actor%20Object%20Reference))
  (|CallParentFunction OtherActor) ; This node is disabled and will not be called.\nDrag off pins to build functionality.
)

(event EventTick
  (params (DeltaSeconds :type Float%20%28single-precision%29))
  (|CallParentFunction DeltaSeconds) ; This node is disabled and will not be called.\nDrag off pins to build functionality.
)

(event EventFire
  (params (IsStart :type Boolean))
  ;[1 1 1] Handle Fire
  (|CallParentFunction IsStart)
  (if IsStart
    (Utilities|FlowControl|DoOnce false :!label _label
      (:Completed
        ;;[1 1 1] Instant first shoot
        (CallFunction|SpawnPrimaryProjectile)
        (Utilities|Time|SetTimerbyEvent (delegate Custom|SpawnPrimaryProjectile) (/ 1.0 (Variables|PrimrayFire|GetPrimrayFireRate)) true)))
    (else
      (Utilities|Time|ClearTimerbyFunctionName 0 "SpawnPrimaryProjectile")
      (goto _label Reset))))

(fn ConstructionScript
  (|CallParentFunction))