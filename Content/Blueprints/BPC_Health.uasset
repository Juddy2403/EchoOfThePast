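; BPC_Health is a component that tracks its owner's health, resetting it to maximum on BeginPlay.
; DoDamage opens a timed invincibility window, calls OnDamage, subtracts clamped damage, and reports whether it hit and whether health is depleted.
; It calls OnDeath only when the hit lowers health to zero, and plays an impact sound on that hit or any non-lethal one.
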(event Custom|ResetHealth
  (Variables|Health|SetCurrentHealth (Variables|Health|GetMaxHealth)))

(event EventBeginPlay
  (CallFunction|ResetHealth))

(event EventTick
  (params (DeltaSeconds :type Float%20%28single-precision%29)))

(fn GetHealthPercentage
  (return (/ (Variables|Health|GetCurrentHealth) (Variables|Health|GetMaxHealth))))

(fn IsDead
  (return (<= (Variables|Health|GetCurrentHealth) 0.0)))

(fn ResetCanbeHit
  (Variables|Default|SetCanBeHit true))

(fn DoDamage
  (params (Amount :type Float%20%28double-precision%29))
  (bind _isdead (CallFunction|IsDead))
  (if (Variables|Default|GetCanBeHit)
    (Variables|Default|SetCanBeHit false)
    (Utilities|Time|SetTimerbyFunctionName 0 "ResetCanBeHit" (Variables|Health|GetInvincibilityTime))
    (Default|CallOnDamage)
    (LocalVariables|SetOriginalHealth (Variables|Health|GetCurrentHealth))
    (bind _output_get (Variables|Health|SetCurrentHealth (Math|Float|Clamp(Float) (- (Variables|Health|GetCurrentHealth) Amount) 0.0 (Variables|Health|GetMaxHealth))))
    ;[1 1 1] Did this DoDamage cause the health to change and drop below 0
    (if _isdead
      (if (> (LocalVariables|GetOriginalHealth) _output_get)
        (Default|CallOnDeath)
        (Audio|SpawnSoundAttached "/Game/Audio/234082__211redman112__lasgun-impact.234082__211redman112__lasgun-impact" (Variables|/Script/Engine.Actor|GetRootComponent (Components|GetOwner)) "None" "0, 0, 0" "0, 0, 0" "KeepRelativeOffset" false 1.0 1.0 0.0 0 0 :!label _label))
      (else
        (goto _label)))
    (return _isdead true)
    (else
      (return (CallFunction|IsDead) false))))