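; Player controller that maps Enhanced Input to BP_PlayerCharacter movement, sprint, dodge, attack, interaction and pause.
; Cursor traces aim attacks and auto-switch melee or ranged weapons based on whether the HUD's 3D cursor is in melee range.
; Middle-mouse drag orbits the spring arm, whose yaw steers movement, and the wheel zooms.
; Listed montages block movement, open dialogue blocks pausing, and non-combat levels change the camera pitch limit.
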(event Custom|PauseMenu
  ;[1 1 1] If no dialogue currently playing
  (bind _foundwidgets (Widget|GetAllWidgetsOfClass "/Game/Blueprints/Widgets/W_Dialogue.W_Dialogue_C" true))
  (if (== (Utilities|Array|Length _foundwidgets) 0)
    (Default|CallOnPauseMenuCommand (not (Game|IsGamePaused)))))

(event Input|EnhancedActionEvents|EnhancedInputActionIA_Interact
  (params (ActionValue :type Boolean) (ElapsedSeconds :type Float%20%28double-precision%29) (TriggeredSeconds :type Float%20%28double-precision%29) (InputAction :type Input%20Action%20Object%20Reference :default "/Game/Input/Actions/IA_Interact.IA_Interact"))
  (bind _interactableobject (Variables|Default|GetInteractableObject))
  ;[0.9922 1 0.5275] Handle interactables
  (:Started
    (if (Utilities|Array|IsNotEmpty _interactableobject)
      (Class|InteractableInterface|Interact(Message) (Utilities|Array|Get(acopy) _interactableobject)))))

(event Input|EnhancedActionEvents|EnhancedInputActionIA_PlayerMovement
  (params (ActionValue :type Vector%202D%20Structure) (ElapsedSeconds :type Float%20%28double-precision%29) (TriggeredSeconds :type Float%20%28double-precision%29) (InputAction :type Input%20Action%20Object%20Reference :default "/Game/Input/Actions/IA_PlayerMovement.IA_PlayerMovement"))
  ;[1 1 1] Add movement input if no rooted animation is playing, taking into account the camera's rotation
  (bind _asbp_player_character (Utilities|Casting|CastToBP_PlayerCharacter (Game|Player|GetPlayerPawn 0)))
  (bind _is_any_playing (Default|IsMontagefromListPlaying _asbp_player_character (Utilities|Array|MakeArray "/Game/Animation/MainCharRetarget/Montages/AM_DodgeMontage.AM_DodgeMontage" "/Game/Animation/MainCharRetarget/Montages/AM_Punch1.AM_Punch1" "/Game/Animation/MainCharRetarget/Montages/AM_Punch2.AM_Punch2" "/Game/Animation/MainCharRetarget/Montages/AM_standing_melee_attack_360_high_Montage.AM_standing_melee_attack_360_high_Montage" "/Game/Animation/MainCharRetarget/Montages/AM_standing_melee_attack_360_low_Montage.AM_standing_melee_attack_360_low_Montage" "/Game/Animation/MainCharRetarget/Montages/AM_standing_melee_attack_downward_Montage.AM_standing_melee_attack_downward_Montage" "/Game/Animation/MainCharRetarget/Montages/AM_standing_melee_attack_horizontal_Montage.AM_standing_melee_attack_horizontal_Montage" "/Game/Animation/MainCharRetarget/Montages/AM_SwordHit.AM_SwordHit")))
  (if (not _is_any_playing)
    (Pawn|Input|AddMovementInput (Pawn|GetControlledPawn) (Math|Vector|Normalize (Math|Vector|RotateVector (Math|Vector|MakeVector (.y ActionValue) (.x ActionValue) 0.0) (Math|Rotator|MakeRotator 0.0 0.0 (Variables|Default|GetSprintArmYaw)))) 1.0 false)))

(event Input|EnhancedActionEvents|EnhancedInputActionIA_Attack
  (params (ActionValue :type Boolean) (ElapsedSeconds :type Float%20%28double-precision%29) (TriggeredSeconds :type Float%20%28double-precision%29) (InputAction :type Input%20Action%20Object%20Reference :default "/Game/Input/Actions/IA_Attack.IA_Attack"))
  (bind _returnvalue (Pawn|GetControlledPawn))
  (bind _asbp_player_character (Utilities|Casting|CastToBP_PlayerCharacter _returnvalue))
  ;[1 1 1] Weapon fire input
  (:Triggered
    ;;[0.4691 0.5478 1] Rotate towards mouse when attacking
    (Transformation|SetActorRelativeRotation _returnvalue (Variables|Default|GetLookAtMouseRotator) :!label _label)
    (Default|Attack _asbp_player_character true))
  (:Started
    (Variables|Default|SetIsAttacking true)
    (goto _label))
  (:Completed
    (Variables|Default|SetIsAttacking false)
    (Default|Attack _asbp_player_character false)))

(event Input|EnhancedActionEvents|EnhancedInputActionIA_PlayerDodge
  (params (ActionValue :type Boolean) (ElapsedSeconds :type Float%20%28double-precision%29) (TriggeredSeconds :type Float%20%28double-precision%29) (InputAction :type Input%20Action%20Object%20Reference :default "/Game/Input/Actions/IA_PlayerDodge.IA_PlayerDodge"))
  ;[1 1 1] Handle dodging
  (:Started
    (Default|Dodge (.AsBP%20Player%20Character (Utilities|Casting|CastToBP_PlayerCharacter (Pawn|GetControlledPawn))))))

(event Input|EnhancedActionEvents|EnhancedInputActionIA_PlayerSprint
  (params (ActionValue :type Boolean) (ElapsedSeconds :type Float%20%28double-precision%29) (TriggeredSeconds :type Float%20%28double-precision%29) (InputAction :type Input%20Action%20Object%20Reference :default "/Game/Input/Actions/IA_PlayerSprint.IA_PlayerSprint"))
  (bind _returnvalue (Pawn|GetControlledPawn))
  (bind _asbp_player_character (Utilities|Casting|CastToBP_PlayerCharacter _returnvalue))
  ;[1 1 1] Handle sprinting
  (:Started
    (Default|StartSprint _asbp_player_character true))
  (:Completed
    (Default|StartSprint _asbp_player_character false)))

(event Input|EnhancedActionEvents|EnhancedInputActionIA_Pause
  (params (ActionValue :type Boolean) (ElapsedSeconds :type Float%20%28double-precision%29) (TriggeredSeconds :type Float%20%28double-precision%29) (InputAction :type Input%20Action%20Object%20Reference :default "/Game/Input/Actions/IA_Pause.IA_Pause"))
  (:Started
    ;[1 1 1] If no dialogue currently playing
    (bind _foundwidgets (Widget|GetAllWidgetsOfClass "/Game/Blueprints/Widgets/W_Dialogue.W_Dialogue_C" true))
    (if (== (Utilities|Array|Length _foundwidgets) 0)
      (Default|CallOnPauseMenuCommand (not (Game|IsGamePaused))))))

(event EventRemoveInteractable
  (params (Interactable :type Object%20Object%20Reference))
  ;[0.9922 1 0.5275] Handle interactables
  (Utilities|Array|RemoveItem (Variables|Default|GetInteractableObject) Interactable))

(event EventAddInteractable
  (params (Interactable :type Object%20Object%20Reference))
  ;[0.9922 1 0.5275] Handle interactables
  (Utilities|Array|Add (Variables|Default|GetInteractableObject) Interactable))

(event Input|MouseEvents|MouseWheelAxis
  (params (AxisValue :type Float%20%28single-precision%29))
  ;[1 1 1] Handle camera zooming with scroll button
  (bind _asbp_player_character (Utilities|Casting|CastToBP_PlayerCharacter (Pawn|GetControlledPawn)))
  (Variables|/Script/Engine.SpringArmComponent|SetTargetArmLength (Variables|/Game/Blueprints/Characters/BP_PlayerCharacter.BP_PlayerCharacter_C|GetSpringArm _asbp_player_character) (Math|Float|Clamp(Float) (+ (Variables|/Script/Engine.SpringArmComponent|GetTargetArmLength (Variables|/Game/Blueprints/Characters/BP_PlayerCharacter.BP_PlayerCharacter_C|GetSpringArm _asbp_player_character)) (* AxisValue (Variables|Default|GetCameraZoomSpeed))) 3e+02 1e+03)))

(event Input|MouseEvents|Mouse2D
  (params (AxisValue :type Vector :default "0, 0, 0"))
  (bind (_hitresult _returnvalue) (Game|Player|GetHitResultUnderCursorbyChannel "TraceTypeQuery3" false))
  ;[1 1 1] If there is mouse movement
  (if (> (Math|Vector|VectorLengthSquared (Math|Vector|MakeVector (.x AxisValue) (.y AxisValue) (.z AxisValue))) 0.0)
    ;[1 1 1] Mouse aiming
    (Utilities|FlowControl|Sequence
      (:then_0
        ;;[1 1 1] Calculate look at rotator
        (if _returnvalue
          (Variables|Default|SetLookAtMouseRotator (Math|Rotator|MakeRotator 0.0 0.0 (.yaw (Math|Rotator|FindLookatRotation (Transformation|GetActorLocation (Pawn|GetControlledPawn)) (.Location (Collision|BreakHitResult _hitresult))))))))
      (:then_1
        (Utilities|FlowControl|Sequence
          (:then_0
            ;[1 1 1] Switch weapon type if it's not attacking, no montage is playing and cursor is in/out of melee range
            (if (Math|Boolean|ANDBoolean _returnvalue (not (Variables|Default|GetIsAttacking)) (not (Class|AnimInstance|IsAnyMontagePlaying (Components|SkeletalMesh|GetAnimInstance (Variables|/Script/Engine.Character|GetMesh (Game|GetPlayerCharacter 0))))))
              (CallFunction|HandleWeaponSwitching)))
          (:then_1
            ;[1 1 1] Rotate camera if MMB is down
            (if (Game|Player|IsInputKeyDown "MiddleMouseButton")
              (CallFunction|HandleCameraRotation (.x AxisValue) (.y AxisValue)))))))))

(fn ConstructionScript)

(fn IsCursorinMeleeRange
  (bind _foundwidgets (Widget|GetAllWidgetsOfClass "/Game/Blueprints/Widgets/W_GameHud.W_GameHud_C" true))
  (bind _returnvalue (Collision|LineTraceByChannel (+ (Variables|/Game/Blueprints/Widgets/W_GameHud.W_GameHud_C|GetCursor3dPos (Utilities|Array|Get(acopy) _foundwidgets)) "0.000000,0.000000,5.000000") (- (Variables|/Game/Blueprints/Widgets/W_GameHud.W_GameHud_C|GetCursor3dPos (Utilities|Array|Get(acopy) _foundwidgets)) "0.000000,0.000000,5.000000") "TraceTypeQuery4" false 0 "None"))
  (return _returnvalue))

(fn HandleWeaponSwitching
  (bind _asbp_player_character (Utilities|Casting|CastToBP_PlayerCharacter (Pawn|GetControlledPawn)))
  (if (CallFunction|IsCursorinMeleeRange)
    ;[1 1 1] Only switch if it's not the current attack type
    (switch Utilities|FlowControl|Switch|SwitchonEDamageType (Variables|/Game/Blueprints/Characters/BP_BaseCharacter.BP_BaseCharacter_C|GetWeaponType _asbp_player_character)
      (:NewEnumerator1
        (Default|SwitchAttackType _asbp_player_character "NewEnumerator0")))
    (else
      (switch Utilities|FlowControl|Switch|SwitchonEDamageType (Variables|/Game/Blueprints/Characters/BP_BaseCharacter.BP_BaseCharacter_C|GetWeaponType _asbp_player_character)
        (:NewEnumerator0
          (Default|SwitchAttackType _asbp_player_character "NewEnumerator1"))))))

(fn HandleCameraRotation
  (params (XAxis :type Float%20%28double-precision%29) (YAxis :type Float%20%28double-precision%29))
  (bind _asbp_player_character (Utilities|Casting|CastToBP_PlayerCharacter (Pawn|GetControlledPawn)))
  (Transformation|SetRelativeRotation (Variables|/Game/Blueprints/Characters/BP_PlayerCharacter.BP_PlayerCharacter_C|GetSpringArm _asbp_player_character) (Math|Rotator|MakeRotator 0.0 (Math|Float|Clamp(Float) (+ (.pitch (Variables|/Script/Engine.SceneComponent|GetRelativeRotation (Variables|/Game/Blueprints/Characters/BP_PlayerCharacter.BP_PlayerCharacter_C|GetSpringArm _asbp_player_character))) (* YAxis (Utilities|Time|GetWorldDeltaSeconds) (Variables|Default|GetRotationSpeed))) -89.0 (Variables|Default|GetMaxCameraPitch)) (+ (.yaw (Variables|/Script/Engine.SceneComponent|GetRelativeRotation (Variables|/Game/Blueprints/Characters/BP_PlayerCharacter.BP_PlayerCharacter_C|GetSpringArm _asbp_player_character))) (* XAxis (Utilities|Time|GetWorldDeltaSeconds) (Variables|Default|GetRotationSpeed)))) false false)
  (Variables|Default|SetSprintArmYaw (.yaw (Variables|/Script/Engine.SceneComponent|GetRelativeRotation (Variables|/Game/Blueprints/Characters/BP_PlayerCharacter.BP_PlayerCharacter_C|GetSpringArm _asbp_player_character)))))

(event Custom|CursorOnPause
  (params (IsPaused :type Boolean))
  (Variables|Default|SetbShowMouseCursor IsPaused))

(event EventBeginPlay
  (bind _returnvalue (Game|GetGameMode))
  (bind _returnvalue_2 (PlayerController|LocalPlayerSubsystems|GetEnhancedInputLocalPlayerSubsystem))
  (bind _returnvalue_3 (Actor|GetComponentbyClass _returnvalue "/Script/EchoOfThePast.PauseHandlerComponent"))
  (Utilities|FlowControl|Sequence
    (:then_0
      ;[1 1 1] Enable default input mapping
      (Utilities|IsValid _returnvalue_2
        (:Is%20Valid
          (Input|AddMappingContext _returnvalue_2 "/Game/Input/IMP_Default.IMP_Default" 0 "(bIgnoreAllPressedKeysUntilRelease=True,bForceImmediately=False,bNotifyUserSettings=False)"))))
    (:then_1
      ;[1 1 1] Used for LookAtCamera function
      (Class|FLookatCamera|InitializeCameraManager self))
    (:then_2
      ;[1 1 1] Set max camera pitch
      (bind _returnvalue_4 (Game|GetCurrentLevelName true))
      (bind _returnvalue_5 (Utilities|GetDataTableRow "/Game/Blueprints/DataTypes/DT_LevelConfig.DT_LevelConfig" (Utilities|String|StringToName _returnvalue_4))
        (:then
          (if (not (.combatenabled _returnvalue_5))
            (Variables|Default|SetMaxCameraPitch -15.0)))))
    (:then_3
      ;[1 1 1] Assign game lost event when the countdown is up
      (Utilities|IsValid _returnvalue_3
        (:Is%20Valid
          (EventDispatchers|BindEventtoOnPaused _returnvalue_3 (delegate Custom|CursorOnPause)))))))