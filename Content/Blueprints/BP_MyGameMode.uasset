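; Game mode that drives enemy spawning, player respawn and score for a game with enemies and projectiles.
; On BeginPlay it starts a looping timer on each BP_EnemySpawner that calls its Spawn function at a per-spawner rate set by EnemiesPerSecondPerSpawner.
; RespawnPlayer destroys all enemies and projectiles, then spawns and possesses a new default pawn at a player start.
; IncreaseScore adds the given amount to Score.
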(event Custom|RespawnPlayer
  (bind _returnvalue (Game|GetPlayerController 0))
  ;[1 1 1] Clear out enemies
  (bind _outactors (Actor|GetAllActorsOfClass "/Game/Blueprints/Characters/BP_EnemyCharacter.BP_EnemyCharacter_C"))
  (for _array_element _outactors
    (Actor|DestroyActor _array_element))
  ;[1 1 1] Clear out projectiles
  (bind _outactors_2 (Actor|GetAllActorsOfClass "/Game/Blueprints/BP_BaseProjectile.BP_BaseProjectile_C"))
  (for _array_element_2 _outactors_2
    (Actor|DestroyActor _array_element_2))
  ;[1 1 1] Player died: respawn
  (bind _returnvalue_2 (Game|SpawnActorfromClass (Variables|Default|GetDefaultPawnClass) (Transformation|GetActorTransform (Class|GameModeBase|FindPlayerStart _returnvalue)) "Undefined" "MultiplyWithRoot" 0 0))
  (Pawn|Possess _returnvalue _returnvalue_2))

(event Custom|IncreaseScore
  (params (ScoreAmount :type Integer))
  ;[1 1 1] Increment score
  (Variables|Default|SetScore (+ ScoreAmount (Variables|Default|GetScore))))

(event EventBeginPlay
  ;[1 1 1] Start spawning enemies
  (bind _outactors (Actor|GetAllActorsOfClass "/Game/Blueprints/BP_EnemySpawner.BP_EnemySpawner_C"))
  (bind _output_get (Variables|EnemySpawns|SetEnemySpawners _outactors))
  (for _array_element _output_get
    (Utilities|Time|SetTimerbyFunctionName _array_element "Spawn" (/ 1.0 (Variables|EnemySpawns|GetEnemiesPerSecondPerSpawner)) true)))

(event EventTick
  (params (DeltaSeconds :type Float%20%28single-precision%29)))

(fn ConstructionScript)