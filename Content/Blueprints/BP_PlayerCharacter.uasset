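; Player character that attacks with a gun or sword, sprints, dodges, and respawns after death.
; Switching attack type replaces the spawned, socket-attached weapon, and attacks call its Fire, with a swing montage for melee.
; Dodge is gated by a cooldown and DoOnce, turns toward movement input and temporarily uses run speed.
; On health component death, it stops movement and firing, then after a delay asks the game mode to respawn and destroys itself.
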(event OnDeath(BPC_Health)
  ;[0.5 0 0.003162] Handle player death
  (Pawn|Components|CharacterMovement|DisableMovement (Variables|Character|GetCharacterMovement))
  (bind _currentweapon (Variables|Default|GetCurrentWeapon)
    (:then
      (Default|Fire _currentweapon false))
    (:else
      _))
  (Utilities|FlowControl|Delay 3.0)
  (bind _asbp_my_game_mode (Utilities|Casting|CastToBP_MyGameMode (Game|GetGameMode)))
  (Default|RespawnPlayer _asbp_my_game_mode)
  (CallFunction|DestroyCurrentWeapon)
  (Actor|DestroyActor))

(event Custom|Dodge
  ;[1 1 1] Dodge
  (if (and (> (- (Utilities|Time|GetGameTimeinSeconds) (Variables|Movement|GetLastTimeDodged)) (Variables|Movement|GetDodgeInterval)) (not (Default|IsDead (Variables|Default|GetBPC_Health))))
    (Variables|Movement|SetLastTimeDodged (Utilities|Time|GetGameTimeinSeconds))
    (Utilities|FlowControl|DoOnce false :!label _label
      (:Completed
        (Variables|/Script/Engine.CharacterMovementComponent|SetMaxWalkSpeed (Variables|Character|GetCharacterMovement) (Variables|Movement|GetRunSpeed))
        (if (CallFunction|IsMoving)
          (Transformation|SetActorRotation (Math|Conversions|RotationFromXVector (Class|Pawn|GetLastMovementInputVector))))
        (Animation|Montage|PlayMontage (Variables|Character|GetMesh) "/Game/ShooterMannequin/Animations/AM_DodgeMontage.AM_DodgeMontage"
          (:OnCompleted
            (Variables|/Script/Engine.CharacterMovementComponent|SetMaxWalkSpeed (Variables|Character|GetCharacterMovement) (Variables|Movement|GetWalkSpeed)))
          (:OnBlendOut
            (goto _label Reset)))))))

(event Custom|StartSprint
  (params (IsStart :type Boolean))
  (bind _charactermovement (Variables|Character|GetCharacterMovement))
  ;[1 1 1] Handle sprint actions
  (if IsStart
    (Variables|/Script/Engine.CharacterMovementComponent|SetMaxWalkSpeed _charactermovement (Variables|Movement|GetRunSpeed))
    (else
      (Variables|/Script/Engine.CharacterMovementComponent|SetMaxWalkSpeed _charactermovement (Variables|Movement|GetWalkSpeed)))))

(event Custom|Attack
  (params (IsStart :type Boolean))
  ;[1 0.5444 0.4409] Handle attack
  (if (not (Default|IsDead (Variables|Default|GetBPC_Health)))
    ;;[1 1 1] If no montage is currently playing
    (if (not (Animation|Montage|MontageIsPlaying (Components|SkeletalMesh|GetAnimInstance (Variables|Character|GetMesh)) 0))
      (switch Utilities|FlowControl|Switch|SwitchonDamageTypeEnum (Variables|Attack|GetAttackType)
        (:NewEnumerator0
          (Animation|Montage|PlayMontage (Variables|Character|GetMesh) "/Game/ShooterMannequin/Animations/AM_SwordHit.AM_SwordHit"
            (:then
              _)))
        (:NewEnumerator1
          _))
      (bind _currentweapon (Variables|Default|GetCurrentWeapon)
        (:then
          (Default|Fire _currentweapon IsStart))
        (:else)))))

(event Custom|SwitchAttackType
  (params (NewParam :type DamageTypeEnum%20Enum :default "NewEnumerator0"))
  ;[1 1 1] Switch attack event
  (bind _output_get (Variables|Attack|SetAttackType NewParam))
  (switch Utilities|FlowControl|Switch|SwitchonDamageTypeEnum _output_get
    (:NewEnumerator0
      (CallFunction|SwitchWeapon (Variables|Attack|GetEquippedSword)))
    (:NewEnumerator1
      (CallFunction|SwitchWeapon (Variables|Attack|GetEquippedGun)))))

(event EventBeginPlay
  ;[0.4462 0.4462 0.4462] Begin play actions
  (|CallParentFunction)
  ;;[1 1 1] Set walk and run speed
  (bind _output_get (Variables|Movement|SetWalkSpeed (Variables|/Script/Engine.CharacterMovementComponent|GetMaxWalkSpeed (Variables|Character|GetCharacterMovement))))
  (Variables|Movement|SetRunSpeed (* _output_get 1.5))
  (CallFunction|SwitchWeapon (Variables|Attack|GetEquippedGun)))

(fn ConstructionScript
  (|CallParentFunction))

(fn IsMoving
  (return (> (Math|Vector|VectorLengthSquared (Transformation|GetVelocity)) 0.0)))

(fn SwitchWeapon
  (params (WeaponRef :type Object%20Class%20Reference))
  ;[1 1 1] If there is a current weapon, destroy it
  (bind _currentweapon (Variables|Default|GetCurrentWeapon)
    (:then
      (Actor|DestroyActor _currentweapon))
    (:else
      _))
  (bind _asbp_base_weapon (Utilities|Casting|CastToBP_BaseWeaponClass (Class|KismetMathLibrary|SelectClass WeaponRef "/Game/Blueprints/BP_BaseWeapon.BP_BaseWeapon_C" (Utilities|IsValidClass WeaponRef))))
  ;[1 1 1] Spawn and attach weapon
  (bind _returnvalue (Game|SpawnActorfromClass _asbp_base_weapon (Math|Transform|MakeTransform "0, 0, 0") "Undefined" "MultiplyWithRoot" 0 0))
  (bind _output_get (Variables|Default|SetCurrentWeapon _returnvalue))
  (Transformation|AttachComponentToComponent _output_get (Variables|Character|GetMesh) (Variables|/Game/Blueprints/BP_BaseWeapon.BP_BaseWeapon_C|GetSocketName _returnvalue) "SnapToTarget" "SnapToTarget" "SnapToTarget" true))