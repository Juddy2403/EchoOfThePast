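; BP_HealPotion is a potion actor that heals the player character when E is pressed nearby.
; It enables input from the first player controller on BeginPlay to receive the key directly.
; On E, if IsCharInSphere is true, it casts to BP_PlayerCharacter, calls Heal on its Health with HealAmount, then destroys itself.
; IsCharInSphere is only read here, as the overlap and tick events are disabled.
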(event EventBeginPlay
  ;[1 1 1] Enable input for processing interaction
  (|CallParentFunction)
  (Input|EnableInput (Game|GetPlayerController 0)))

(event Collision|EventActorBeginOverlap
  (params (OtherActor :type Actor%20Object%20Reference))
  (|CallParentFunction OtherActor) ; This node is disabled and will not be called.\nDrag off pins to build functionality.
)

(event EventTick
  (params (DeltaSeconds :type Float%20%28single-precision%29))
  (|CallParentFunction DeltaSeconds) ; This node is disabled and will not be called.\nDrag off pins to build functionality.
)

(event Input|KeyboardEvents|E
  (params (Key :type Key%20Structure :default "None"))
  ;[0.3896 1 0.4575] Heal character when pressing E
  (:Pressed
    (if (Variables|Default|GetIsCharInSphere)
      (bind _asbp_player_character (Utilities|Casting|CastToBP_PlayerCharacter (Game|GetPlayerCharacter 0)))
      (Class|Health|Heal (Variables|/Game/Blueprints/BP_BaseCharacter.BP_BaseCharacter_C|GetHealth _asbp_player_character) (Variables|Default|GetHealAmount))
      (Actor|DestroyActor))))

(fn ConstructionScript
  (|CallParentFunction))