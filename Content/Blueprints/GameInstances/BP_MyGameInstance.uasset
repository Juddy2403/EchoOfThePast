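; Game instance that carries player stats and the remaining timer value across level loads.
; SetPlayerStats caches the pawn's stats through interface messages.
; A one-shot binding to the level-loaded event waits a tick, pushes those stats to the pawn and RemainingTime to BP_MyGameMode's timer component, then unbinds.
; GetPlayerModifiers returns zero for health, speed and damage modifiers.
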(event Custom|SetPlayerStats
  ;[1 1 1] Update player stats
  (bind _returnvalue (Class|PlayerStatsInterface|GetPlayerStats(Message) (Game|Player|GetPlayerPawn 0)))
  (Variables|Default|SetPlayerStats _returnvalue))

(event Custom|SetPlayerGIStats
  ;[1 1 1] Retrieve player stats and timer from last level
  (Utilities|FlowControl|DelayUntilNextTick)
  (Class|PlayerStatsInterface|SetPlayerStats(Message) (Game|Player|GetPlayerPawn 0) (Variables|Default|GetPlayerStats))
  (bind _asbp_my_game_mode (Utilities|Casting|CastToBP_MyGameMode (Game|GetGameMode)))
  (Variables|/Game/Blueprints/Components/BP_Timer_AC.BP_Timer_AC_C|SetRemainingTime (Variables|/Game/Blueprints/GameModes/BP_MyGameMode.BP_MyGameMode_C|GetBP_Timer_AC _asbp_my_game_mode) (Variables|Default|GetRemainingTime))
  (EventDispatchers|UnbindEventfromOnLevelLoaded (delegate Custom|SetPlayerGIStats)))

(event Custom|BindSetPlayerStatsEvent
  ;[1 1 1] Retrieve player stats and timer from last level
  (EventDispatchers|BindEventtoOnLevelLoaded (delegate Custom|SetPlayerGIStats)))

(fn GetPlayerModifiers
  (return 0.0 0.0 0.0))