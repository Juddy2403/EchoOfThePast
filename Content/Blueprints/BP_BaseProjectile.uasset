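; Base projectile Blueprint that deals damage to what it strikes and then destroys itself.
; Collision hit and begin-overlap events both feed ProcessCollision, which skips invalid actors and those carrying IgnoreTag.
; Damage goes through BPI_Damageable messages to the actor and its implementing components, rechecking actor validity during the component loop.
; An older direct BPC_Health damage path remains in the event graph but is disconnected.
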(event OnComponentHit(Collision)
  (params (HitComponent :type Primitive%20Component%20Object%20Reference) (OtherActor :type Actor%20Object%20Reference) (OtherComp :type Primitive%20Component%20Object%20Reference) (NormalImpulse :type Vector :default "0, 0, 0") (Hit :type Hit%20Result%20Structure%20%28by%20ref%29))
  (CallFunction|ProcessCollision OtherActor))

(event OnComponentBeginOverlap(Collision)
  (params (OverlappedComponent :type Primitive%20Component%20Object%20Reference) (OtherActor :type Actor%20Object%20Reference) (OtherComp :type Primitive%20Component%20Object%20Reference) (OtherBodyIndex :type Integer) (bFromSweep :type Boolean) (SweepResult :type Hit%20Result%20Structure%20%28by%20ref%29))
  (CallFunction|ProcessCollision OtherActor))

(event EventBeginPlay)

(event Collision|EventActorBeginOverlap
  (params (OtherActor :type Actor%20Object%20Reference)))

(event EventTick
  (params (DeltaSeconds :type Float%20%28single-precision%29)))

(fn ConstructionScript)

(fn ProcessCollision
  (params (OtherActor :type Actor%20Object%20Reference))
  (bind _returnvalue (Class|Actor|GetComponentsbyInterface OtherActor "/Game/Blueprints/BPI_Damageable.BPI_Damageable_C"))
  ;[1 1 1] Check if we hit an actor
  (Utilities|IsValid OtherActor
    (:Is%20Valid
      (if (not (Actor|ActorHasTag OtherActor (Variables|Default|GetIgnoreTag)))
        (Utilities|FlowControl|Sequence
          (:then_0
            (if (Utilities|DoesObjectImplementInterface OtherActor "/Game/Blueprints/BPI_Damageable.BPI_Damageable_C")
              (Class|BPIDamageable|DoDamage(Message) OtherActor (Variables|Default|GetDamageAmount))))
          (:then_1
            (Utilities|IsValid OtherActor
              (:Is%20Valid
                ;[1 1 1] Get all Components that implement the BPI_Damageable interfere and do damage
                (bind _index (Utilities|FlowControl|ForLoopwithBreak 0 (- (Utilities|Array|Length _returnvalue) -1) :!label _label)
                  (:LoopBody
                    (Class|BPIDamageable|DoDamage(Message) (Utilities|Array|Get(acopy) _returnvalue _index) (Variables|Default|GetDamageAmount))
                    (Utilities|IsValid OtherActor
                      (:Is%20Not%20Valid
                        (goto _label Break))))))))
          (:then_2
            (Actor|DestroyActor)))))))