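; Enemy spawner actor that creates a BP_EnemyCharacter with AI whenever its Spawn event is called.
; Spawn does nothing once the live enemy count exceeds MaxAmountOfActiveEnemies from BP_MyGameMode, using zero as the limit if that cast fails.
; UseSpawnVolume selects between a random point inside the SpawnVolume box and the actor's root location, always using the root's rotation.
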(event Custom|Spawn
  (bind _returnvalue (Game|GetGameMode))
  (bind _defaultsceneroot (Variables|Default|GetDefaultSceneRoot))
  (bind _spawnvolume (Variables|Default|GetSpawnVolume))
  (bind (_asbp_my_game_mode _bsuccess) (Utilities|Casting|CastToBP_MyGameMode _returnvalue))
  ;[1 1 1] Limit the nr of spawns
  (bind _outactors (Actor|GetAllActorsOfClass "/Game/Blueprints/Characters/BP_EnemyCharacter.BP_EnemyCharacter_C"))
  (if (not (> (Utilities|Array|Length _outactors) (Math|Integer|SelectInt (Variables|/Game/Blueprints/BP_MyGameMode.BP_MyGameMode_C|GetMaxAmountOfActiveEnemies _asbp_my_game_mode) 0 _bsuccess)))
    (AI|SpawnAIFromClass "/Game/Blueprints/Characters/BP_EnemyCharacter.BP_EnemyCharacter_C" 0 (Math|Vector|SelectVector (Math|Random|RandomPointinBoundingBox (Transformation|GetWorldLocation _spawnvolume) (Components|Box|GetScaledBoxExtent _spawnvolume)) (Transformation|GetWorldLocation _defaultsceneroot) (Variables|Default|GetUseSpawnVolume)) (Transformation|GetWorldRotation _defaultsceneroot) false 0)))

(event EventBeginPlay)

(event Collision|EventActorBeginOverlap
  (params (OtherActor :type Actor%20Object%20Reference)))

(event EventTick
  (params (DeltaSeconds :type Float%20%28single-precision%29)))

(fn ConstructionScript)