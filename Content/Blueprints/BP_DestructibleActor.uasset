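; Destructible actor that reacts to its health component by flashing red when damaged and destroying itself on death.
; On damage it creates a dynamic material instance on the mesh, caches its Color parameter, and a timeline blends between red and that color before restoring it.
; A DoOnce gate, reset when the timeline finishes, ignores further hits during an active flicker.
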(event OnDeath(BPC_Health)
  (Actor|DestroyActor))

(event OnDamage(BPC_Health)
  (Utilities|FlowControl|DoOnce false :!label _label
    (:Completed
      (bind _returnvalue (Rendering|Material|CreateDynamicMaterialInstance (Variables|Default|GetMesh) 0 0 "None" :!class /Script/Engine.PrimitiveComponent))
      (Utilities|FlowControl|Sequence
        (:then_0
          (bind _returnvalue_2 (Rendering|Material|GetVectorParameterValue _returnvalue "Color" :!class /Script/Engine.MaterialInstanceDynamic)))
        (:then_1
          (bind _flickerstate (Timeline|FlickerTimeline PlayFromStart)
            (:Update
              (Rendering|Material|SetVectorParameterValue _returnvalue "Color" (Math|Color|Lerp(LinearColor) "(R=1.000000,G=0.010132,B=0.000000,A=1.000000)" _returnvalue_2 _flickerstate) :!class /Script/Engine.MaterialInstanceDynamic))
            (:Finished
              (Rendering|Material|SetVectorParameterValue _returnvalue "Color" _returnvalue_2 :!class /Script/Engine.MaterialInstanceDynamic)
              (goto _label Reset))))))))

(fn ConstructionScript)