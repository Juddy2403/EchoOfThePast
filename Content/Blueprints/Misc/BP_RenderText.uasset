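; Placeable world text actor that appears only while the player character is within a sphere trigger.
; Sphere overlaps with BP_PlayerCharacter show or hide the TextRender and set a flag that lets Tick turn it to face the camera.
; The construction script applies the exposed text, size, offsets and trigger radius for per-instance setup.
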(event OnComponentBeginOverlap(Sphere)
  (params (OverlappedComponent :type Primitive%20Component%20Object%20Reference) (OtherActor :type Actor%20Object%20Reference) (OtherComp :type Primitive%20Component%20Object%20Reference) (OtherBodyIndex :type Integer) (bFromSweep :type Boolean) (SweepResult :type Hit%20Result%20Structure%20%28by%20ref%29))
  (Utilities|Casting|CastToBP_PlayerCharacter OtherActor)
  (Variables|Default|SetIsCharInSphere true)
  (Development|SetHiddeninGame (Variables|Default|GetTextRender) false false))

(event OnComponentEndOverlap(Sphere)
  (params (OverlappedComponent :type Primitive%20Component%20Object%20Reference) (OtherActor :type Actor%20Object%20Reference) (OtherComp :type Primitive%20Component%20Object%20Reference) (OtherBodyIndex :type Integer))
  (Utilities|Casting|CastToBP_PlayerCharacter OtherActor)
  (Variables|Default|SetIsCharInSphere false)
  (Development|SetHiddeninGame (Variables|Default|GetTextRender) true false))

(event EventBeginPlay)

(event Collision|EventActorBeginOverlap
  (params (OtherActor :type Actor%20Object%20Reference)))

(event EventTick
  (params (DeltaSeconds :type Float%20%28single-precision%29))
  (if (Variables|Default|GetIsCharInSphere)
    (Class|FLookatCamera|LookatCamera (Variables|Default|GetTextRender) false false)))

(fn ConstructionScript
  (bind _sphere (Variables|Default|GetSphere))
  (bind _textrender (Variables|Default|GetTextRender))
  (Components|Sphere|SetSphereRadius _sphere (Variables|Default|GetSphereRadius) true)
  (Transformation|AddLocalOffset _sphere (Variables|Default|GetSphereOffset) false false)
  (Rendering|Components|TextRender|SetText _textrender (Variables|Default|GetTextToDisplay))
  (Transformation|AddLocalOffset _textrender (Variables|Default|GetTextOffset) false false)
  (Rendering|Components|TextRender|SetWorldSize _textrender (Variables|Default|GetTextSize)))