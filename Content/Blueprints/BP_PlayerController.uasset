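; Player controller for a cursor-aimed character that sets up the input mapping, HUD and camera manager on BeginPlay.
; Enhanced Input events drive world-axis movement and forward attack, sprint and dodge to BP_PlayerCharacter.
; Mouse input traces under the cursor to store a yaw-only look-at rotation, which the pawn snaps to while firing.
; Cursor distance from the pawn also auto-switches between melee and ranged attacks.
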(event Input|EnhancedActionEvents|EnhancedInputActionIA_PlayerMovement
  (params (ActionValue :type Vector%202D%20Structure) (ElapsedSeconds :type Float%20%28double-precision%29) (TriggeredSeconds :type Float%20%28double-precision%29) (InputAction :type Input%20Action%20Object%20Reference :default "/Game/Input/Actions/IA_PlayerMovement.IA_PlayerMovement"))
  ;[1 1 1] Add movement input
  (Pawn|Input|AddMovementInput (Pawn|GetControlledPawn) (Math|Vector|ClampVectorSize (Math|Vector|MakeVector (.y ActionValue) (.x ActionValue) 0.0) 0.0 1.0) 1.0 false))

(event Input|EnhancedActionEvents|EnhancedInputActionIA_FirePrimary
  (params (ActionValue :type Boolean) (ElapsedSeconds :type Float%20%28double-precision%29) (TriggeredSeconds :type Float%20%28double-precision%29) (InputAction :type Input%20Action%20Object%20Reference :default "/Game/Input/Actions/IA_FirePrimary.IA_FirePrimary"))
  (bind _returnvalue (Pawn|GetControlledPawn))
  (bind _asbp_player_character (Utilities|Casting|CastToBP_PlayerCharacter _returnvalue))
  ;[1 1 1] Weapon fire input
  (:Triggered
    ;;[0.4691 0.5478 1] Rotate towards mouse when attacking
    (Transformation|SetActorRelativeRotation _returnvalue (Variables|Default|GetLookAtMouseRotator) :!label _label)
    (Default|Attack _asbp_player_character true))
  (:Started
    (Variables|Default|SetIsAttacking true)
    (goto _label))
  (:Completed
    (Variables|Default|SetIsAttacking false)
    (Default|Attack _asbp_player_character false)))

(event Input|EnhancedActionEvents|EnhancedInputActionIA_PlayerDodge
  (params (ActionValue :type Boolean) (ElapsedSeconds :type Float%20%28double-precision%29) (TriggeredSeconds :type Float%20%28double-precision%29) (InputAction :type Input%20Action%20Object%20Reference :default "/Game/Input/Actions/IA_PlayerDodge.IA_PlayerDodge"))
  ;[1 1 1] Handle dodging
  (:Started
    (Default|Dodge (.AsBP%20Player%20Character (Utilities|Casting|CastToBP_PlayerCharacter (Pawn|GetControlledPawn))))))

(event Input|EnhancedActionEvents|EnhancedInputActionIA_PlayerSprint
  (params (ActionValue :type Boolean) (ElapsedSeconds :type Float%20%28double-precision%29) (TriggeredSeconds :type Float%20%28double-precision%29) (InputAction :type Input%20Action%20Object%20Reference :default "/Game/Input/Actions/IA_PlayerSprint.IA_PlayerSprint"))
  (bind _returnvalue (Pawn|GetControlledPawn))
  (bind _asbp_player_character (Utilities|Casting|CastToBP_PlayerCharacter _returnvalue))
  ;[1 1 1] Handle sprinting
  (:Started
    (Default|StartSprint _asbp_player_character true))
  (:Completed
    (Default|StartSprint _asbp_player_character false)))

(event EventBeginPlay
  (bind _returnvalue (PlayerController|LocalPlayerSubsystems|GetEnhancedInputLocalPlayerSubsystem))
  (Utilities|FlowControl|Sequence
    (:then_0
      ;[1 1 1] Enable default input mapping
      (Utilities|IsValid _returnvalue
        (:Is%20Valid
          (Input|AddMappingContext _returnvalue "/Game/Input/IMP_Default.IMP_Default" 0 "(bIgnoreAllPressedKeysUntilRelease=True,bForceImmediately=False,bNotifyUserSettings=False)"))))
    (:then_1
      ;[1 1 1] Add hud
      (bind _returnvalue_2 (UserInterface|CreateWidget "/Game/Blueprints/BPW_GameHud.BPW_GameHud_C" self))
      (UserInterface|Viewport|AddtoViewport _returnvalue_2 0))
    (:then_2
      (Class|FLookatCamera|InitializeCameraManager self))))

(event Input|MouseEvents|Mouse2D
  (params (AxisValue :type Vector :default "0, 0, 0"))
  (bind (_hitresult _returnvalue) (Game|Player|GetHitResultUnderCursorbyChannel "TraceTypeQuery1" true))
  (bind _returnvalue_2 (Pawn|GetControlledPawn))
  (bind _location (Collision|BreakHitResult _hitresult))
  ;[1 1 1] Mouse aiming
  ;;[1 1 1] Detect mouse movement
  (Utilities|FlowControl|Sequence
    (:then_0
      ;;[1 1 1] Calculate look at rotator
      (if _returnvalue
        (Variables|Default|SetLookAtMouseRotator (Math|Rotator|MakeRotator 0.0 0.0 (.yaw (Math|Rotator|FindLookatRotation (Transformation|GetActorLocation (Pawn|GetControlledPawn)) _location))))))
    (:then_1
      ;[1 1 1] If there is mouse movement
      (if (> (Math|Vector|VectorLengthSquared AxisValue) 0.0)
        ;[1 1 1] Switch attack
        ;;[1 1 1] If hit result valid
        (if _returnvalue
          (bind _asbp_player_character (Utilities|Casting|CastToBP_PlayerCharacter _returnvalue_2))
          (if (> (Variables|Default|GetMeleeMouseRange) (Math|Vector|VectorLength (- _location (Transformation|GetActorLocation _returnvalue_2))))
            (switch Utilities|FlowControl|Switch|SwitchonDamageTypeEnum (Variables|/Game/Blueprints/BP_PlayerCharacter.BP_PlayerCharacter_C|GetAttackType _asbp_player_character)
              (:NewEnumerator1
                (Default|SwitchAttackType _asbp_player_character "NewEnumerator0")))
            (else
              (switch Utilities|FlowControl|Switch|SwitchonDamageTypeEnum (Variables|/Game/Blueprints/BP_PlayerCharacter.BP_PlayerCharacter_C|GetAttackType _asbp_player_character)
                (:NewEnumerator0
                  (Default|SwitchAttackType _asbp_player_character "NewEnumerator1"))))))))))

(fn ConstructionScript)