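; Actor component that shows floating damage numbers, or "Miss" for zero or negative damage, as Niagara effects at a given location.
; InitData derives the text, crit-based scale, hit or miss tint, and canvas size from text length.
; DrawFloatingDamage draws that text into a runtime render target, wraps it in a dynamic material, and spawns NS_FloatingDamage fed with material, tint and dimensions.
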(event EventBeginPlay)

(event EventTick
  (params (DeltaSeconds :type Float%20%28single-precision%29)))

(fn InitData
  (params (DamageAmount :type Float%20%28double-precision%29) (IsCrit :type Boolean))
  (bind _returnvalue (> DamageAmount 0.0))
  (if IsCrit
    (Variables|Default|SetTextScale "(X=1.500000,Y=1.500000)")
    (else
      (Variables|Default|SetTextScale "(X=0.700000,Y=0.700000)")))
  (bind _output_get (Variables|Default|SetText (Utilities|String|SelectString (Utilities|String|ToString(Integer) (Class|KismetMathLibrary|ToInt64(Float) DamageAmount)) "Miss" _returnvalue)))
  (bind _output_get_2 (Variables|Default|SetDimensions (Math|Vector2D|MakeVector2D (* (Math|Conversions|ToFloat(Integer) (Utilities|String|Len _output_get)) (Variables|Default|GetDimensionsMultiplier)) (Variables|Default|GetDimensionsMultiplier))))
  (Variables|Default|SetTextTint (Math|Color|SelectColor "(R=1.000000,G=0.000000,B=0.000000,A=1.000000)" "(R=1.000000,G=0.873327,B=0.000000,A=1.000000)" _returnvalue))
  (Variables|Default|SetOffset (/ _output_get_2 2.0)))

(fn DrawFloatingDamage
  (params (Location :type Vector))
  (bind _dimensions (Variables|Default|GetDimensions))
  (Utilities|FlowControl|Sequence
    (:then_0
      (Utilities|FlowControl|Sequence
        (:then_0
          (bind _returnvalue (Rendering|CreateRenderTarget2D (Math|Float|Truncate (.x _dimensions)) (Math|Float|Truncate (.y _dimensions)) "RTF_R8"))
          (Variables|Default|SetRenderTarget _returnvalue)
          (bind _returnvalue_2 (Rendering|Material|CreateDynamicMaterialInstance "/Game/Materials/M_DamageWidget.M_DamageWidget" "None" "None" :!class /Script/Engine.KismetMaterialLibrary))
          (bind _output_get (Variables|Default|SetMaterial _returnvalue_2))
          (Rendering|Material|SetTextureParameterValue _output_get "RT_FloatingDamage" (Variables|Default|GetRenderTarget)))
        (:then_1
          (bind (_canvas _size _context) (Rendering|BeginDrawCanvastoRenderTarget (Variables|Default|GetRenderTarget)))
          (Variables|Default|SetTempCanvas _canvas)
          (Variables|Default|SetTempCanvasContext _context)
          (HUD|DrawText (Variables|Default|GetTempCanvas) "/Engine/EngineFonts/RobotoDistanceField.RobotoDistanceField" (Variables|Default|GetText) (Variables|Default|GetOffset) (Variables|Default|GetTextScale) "(R=1.000000,G=1.000000,B=1.000000,A=1.000000)" 0.0 "(R=0.000000,G=0.000000,B=0.000000,A=1.000000)" "(X=1.000000,Y=1.000000)" true true false "(R=0.000000,G=0.000000,B=0.000000,A=1.000000)")
          (Rendering|EndDrawCanvastoRenderTarget (Variables|Default|GetTempCanvasContext)))))
    (:then_1
      (Utilities|FlowControl|Sequence
        (:then_0
          (bind _returnvalue_3 (Niagara|SpawnSystematLocation "/Game/Blueprints/Particles/NS_FloatingDamage.NS_FloatingDamage" Location))
          (Variables|Default|SetTempVFX _returnvalue_3))
        (:then_1
          (Niagara|SetNiagaraVariable(LinearColor) (Variables|Default|GetTempVFX) "TextTint" (Variables|Default|GetTextTint))
          (Class|NiagaraComponent|SetVariableVec2 (Variables|Default|GetTempVFX) "TextDimensions" (Variables|Default|GetDimensions))
          (Class|NiagaraComponent|SetVariableMaterial (Variables|Default|GetTempVFX) "Material" (Variables|Default|GetMaterial)))))))