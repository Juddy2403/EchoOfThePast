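; BP_DisplayText_AC is a component that shows a text message on screen for a limited time.
; On BeginPlay it creates a W_DisplayText widget, sets its Text and adds it to the viewport hidden.
; ShowText makes the widget visible, waits for Duration, then hides it again, ignoring calls made while the text is already showing.
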(event Custom|ShowText
  (bind _widget (Variables|Default|GetWidget))
  ;[1 1 1] If not visible already
  ;[1 1 1] Show for an amount of time, then collapse again
  (if (not (Utilities|Enum|Equal(Enum) (Widget|GetVisibility (Variables|Default|GetWidget)) "Visible"))
    (Widget|SetVisibility _widget "Visible")
    (Utilities|FlowControl|Delay (Variables|Default|GetDuration))
    (Widget|SetVisibility _widget "Hidden")))

(event EventBeginPlay
  ;[1 1 1] Initialize widget and set it to hidden
  (bind _returnvalue (UserInterface|CreateWidget "/Game/Blueprints/Widgets/W_DisplayText.W_DisplayText_C"))
  (bind _output_get (Variables|Default|SetWidget _returnvalue))
  (Default|SetDisplayText _output_get (Variables|Default|GetText))
  (Widget|SetVisibility _output_get "Hidden")
  (UserInterface|Viewport|AddtoViewport (Variables|Default|GetWidget) 0))

(event EventTick
  (params (DeltaSeconds :type Float%20%28single-precision%29)))