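; BP_Music_AC is an actor component that plays background music in levels flagged for combat.
; On BeginPlay it looks up the current level name in DT_LevelConfig and uses the CombatEnabled flag to decide whether to play.
; When allowed and Music is valid, it creates and starts a 2D sound at the set volume.
; EnableSound pauses or resumes that sound, only if playback was allowed.
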(event Custom|EnableSound
  (params (Enable :type Boolean))
  (bind _soundsource (Variables|Default|GetSoundSource))
  (if (Variables|Default|GetShouldPlay)
    (if Enable
      (Class|AudioComponent|SetPaused _soundsource false)
      (else
        (Class|AudioComponent|SetPaused _soundsource true)))))

(event EventBeginPlay
  (bind _returnvalue (Game|GetCurrentLevelName true))
  (bind _returnvalue_2 (Utilities|GetDataTableRow "/Game/Blueprints/DataTypes/DT_LevelConfig.DT_LevelConfig" (Utilities|String|StringToName _returnvalue))
    (:then
      (bind _output_get (Variables|Default|SetShouldPlay (.combatenabled _returnvalue_2)))
      (if _output_get
        (bind _music (Variables|Default|GetMusic)
          (:then
            (bind _returnvalue_3 (Audio|CreateSound2D _music (Variables|Default|GetVolume%20Multiplier) 1.0 0.0 0))
            (bind _output_get_2 (Variables|Default|SetSoundSource _returnvalue_3))
            (Audio|Components|Audio|Play _output_get_2 0.0))
          (:else))))))

(event EventTick
  (params (DeltaSeconds :type Float%20%28single-precision%29)))