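; BP_Timer_AC is a countdown timer component that starts from a configurable duration.
; BeginPlay copies the duration into RemainingTime, and each Tick, commented as once per second, subtracts one and fires TimeUpdated.
; Once time runs out, OnTimeUp fires on every subsequent Tick, as nothing in the graph stops it.
; GetRemainingTime formats the remaining count as minutes:seconds text.
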(event EventBeginPlay
  (Variables|Default|SetRemainingTime (Variables|Default|GetTimerDuration)))

(event EventTick
  (params (DeltaSeconds :type Float%20%28single-precision%29))
  ;[1 1 1] Updates every second
  (if (> (Variables|Default|GetRemainingTime) 0)
    (Variables|Default|SetRemainingTime (- (Variables|Default|GetRemainingTime) 1))
    (Default|CallTimeUpdated)
    (else
      (Default|CallOnTimeUp))))

(fn GetRemainingTime
  (bind _remainingtime (Variables|Default|GetRemainingTime))
  (return (Utilities|Text|FormatText "{Minutes}:{Seconds}" (Utilities|Text|ToText(Integer) (/ _remainingtime 60) false true 2) (Utilities|Text|ToText(Integer) (Math|Integer|%(Integer) _remainingtime 60) false true 2))))