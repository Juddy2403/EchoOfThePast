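; Dialogue component that shows a character's lines in a W_Dialogue widget with matching 2D voice audio.
; The first Talk call creates the widget and pauses the game through the GameMode's PauseHandlerComponent; later calls step through the parallel text and audio arrays.
; Advancing stops the previous tracked clip, though the first line's audio is untracked.
; After the last line it removes the widget, resets, and, given a pause handler, unpauses and fires OnDialogueOver.
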(event Custom|StopPreviousAudio
  (bind _currentlyplayedaudio (Variables|Default|GetCurrentlyPlayedAudio)
    (:then
      (if (Audio|Components|Audio|IsPlaying _currentlyplayedaudio)
        (Audio|Components|Audio|Stop _currentlyplayedaudio)))
    (:else)))

(event EventTalk
  (bind _returnvalue (Game|GetGameMode))
  (bind _returnvalue_2 (Game|GetGameMode))
  (bind _dialoguetext (Variables|Default|GetDialogueText))
  (bind _returnvalue_3 (Actor|GetComponentbyClass _returnvalue "/Script/EchoOfThePast.PauseHandlerComponent"))
  (bind _returnvalue_4 (Actor|GetComponentbyClass _returnvalue_2 "/Script/EchoOfThePast.PauseHandlerComponent"))
  (Utilities|IsValid (Variables|Default|GetWidget)
    (:Is%20Valid
      (bind _result (Math|Integer|IncrementInt (Variables|Default|GetLineIdx))
        (:%20%20
          (if (>= _result (Utilities|Array|Length _dialoguetext))
            ;[1 1 1] When dialogue is over, remove widget
            (Widget|RemovefromParent (Variables|Default|GetWidget))
            (Variables|Default|SetWidget 0)
            (Variables|Default|SetLineIdx 0)
            (Utilities|IsValid _returnvalue_3
              (:Is%20Valid
                (Class|PauseHandlerComponent|PauseGame _returnvalue_3 false)
                (Default|CallOnDialogueOver)))
            (else
              ;[1 1 1] Update dialogue line
              (Default|SetDialogueText (Variables|Default|GetWidget) (Utilities|Array|Get(acopy) _dialoguetext _result))
              (CallFunction|StopPreviousAudio)
              (bind _returnvalue_5 (Audio|SpawnSound2D (Utilities|Array|Get(acopy) (Variables|Default|GetDialogueAudio) _result) 1.0 1.0 0.0 0))
              (Variables|Default|SetCurrentlyPlayedAudio _returnvalue_5))))))
    (:Is%20Not%20Valid
      ;[1 1 1] Create dialogue widget if it's not created yet
      (bind _returnvalue_6 (UserInterface|CreateWidget "/Game/Blueprints/Widgets/W_Dialogue.W_Dialogue_C"))
      (bind _output_get (Variables|Default|SetWidget _returnvalue_6))
      (UserInterface|Viewport|AddtoViewport _output_get 0)
      (Variables|/Game/Blueprints/Widgets/W_Dialogue.W_Dialogue_C|SetCharName _output_get (Variables|Default|GetCharName))
      (Default|SetDialogueText _output_get (Utilities|Array|Get(acopy) (Variables|Default|GetDialogueText)))
      (Audio|PlaySound2D (Utilities|Array|Get(acopy) (Variables|Default|GetDialogueAudio)) 1.0 1.0 0.0 0 0)
      (Utilities|IsValid _returnvalue_4
        (:Is%20Valid
          (Class|PauseHandlerComponent|PauseGame _returnvalue_4 true))))))