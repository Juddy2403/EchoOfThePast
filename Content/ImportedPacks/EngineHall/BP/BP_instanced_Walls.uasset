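; Construction-time tool actor that builds a wall from a grid of instances of one configurable static mesh.
; The construction script assigns Mesh01 to the instanced mesh component, then adds Rows × Columns local-space instances in the XZ plane with adjustable spacing, offset and uniform scale.
; Integer division and modulo on the index place the grid, so Rows counts along X and Columns up Z.
; The event graph has no runtime logic.
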(event EventBeginPlay)

(event Collision|EventActorBeginOverlap
  (params (OtherActor :type Actor%20Object%20Reference)))

(event EventTick
  (params (DeltaSeconds :type Float%20%28single-precision%29)))

(fn ConstructionScript
  ;[1 1 1] Set used Mesh
  (Components|StaticMesh|SetStaticMesh (Variables|Default|GetMesh) (Variables|Default|GetMesh_01))
  ;[1 1 1] Setting number of instances
  (for _index (range 0 (- (* (Variables|Meshes|Getrows) (Variables|Meshes|GetColumns)) 1))
    ;[1 1 1] Adding mesh instances
    (Components|InstancedStaticMesh|AddInstance (Variables|Default|GetMesh) (Math|Transform|MakeTransform (+ (Variables|Meshes|GetLocation%20offset) (.Location (Math|Transform|BreakTransform (Math|Conversions|ToTransform(Vector) (Math|Vector|MakeVector (Math|Conversions|ToFloat(Integer) (* (/ _index (Variables|Meshes|GetColumns)) (Variables|Meshes|GetMeshes%20distance%20Columns))) 0.0 (Math|Conversions|ToFloat(Integer) (* (Math|Integer|%(Integer) _index (Variables|Meshes|GetColumns)) (Variables|Meshes|GetMeshes%20distance%20Rows)))))))) (.Rotation (Math|Transform|BreakTransform (Math|Conversions|ToTransform(Vector) (Math|Vector|MakeVector (Math|Conversions|ToFloat(Integer) (* (/ _index (Variables|Meshes|GetColumns)) (Variables|Meshes|GetMeshes%20distance%20Columns))) 0.0 (Math|Conversions|ToFloat(Integer) (* (Math|Integer|%(Integer) _index (Variables|Meshes|GetColumns)) (Variables|Meshes|GetMeshes%20distance%20Rows))))))) (Math|Vector|MakeVector (* (.X (Math|Vector|BreakVector (.Scale (Math|Transform|BreakTransform (Math|Conversions|ToTransform(Vector) (Math|Vector|MakeVector (Math|Conversions|ToFloat(Integer) (* (/ _index (Variables|Meshes|GetColumns)) (Variables|Meshes|GetMeshes%20distance%20Columns))) 0.0 (Math|Conversions|ToFloat(Integer) (* (Math|Integer|%(Integer) _index (Variables|Meshes|GetColumns)) (Variables|Meshes|GetMeshes%20distance%20Rows))))))))) (Variables|Meshes|GetScale)) (* (.Y (Math|Vector|BreakVector (.Scale (Math|Transform|BreakTransform (Math|Conversions|ToTransform(Vector) (Math|Vector|MakeVector (Math|Conversions|ToFloat(Integer) (* (/ _index (Variables|Meshes|GetColumns)) (Variables|Meshes|GetMeshes%20distance%20Columns))) 0.0 (Math|Conversions|ToFloat(Integer) (* (Math|Integer|%(Integer) _index (Variables|Meshes|GetColumns)) (Variables|Meshes|GetMeshes%20distance%20Rows))))))))) (Variables|Meshes|GetScale)) (* (.Z (Math|Vector|BreakVector (.Scale (Math|Transform|BreakTransform (Math|Conversions|ToTransform(Vector) (Math|Vector|MakeVector (Math|Conversions|ToFloat(Integer) (* (/ _index (Variables|Meshes|GetColumns)) (Variables|Meshes|GetMeshes%20distance%20Columns))) 0.0 (Math|Conversions|ToFloat(Integer) (* (Math|Integer|%(Integer) _index (Variables|Meshes|GetColumns)) (Variables|Meshes|GetMeshes%20distance%20Rows))))))))) (Variables|Meshes|GetScale)))) false)))